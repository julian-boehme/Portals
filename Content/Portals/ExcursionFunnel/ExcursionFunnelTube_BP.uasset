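; Anti-gravity tube segment of an Excursion Funnel that carries the player and physics objects along its axis.
; On overlap, if ParentFunnel is enabled, it disables gravity, zeroes velocity, snaps non-portal actors to the centerline and applies force scaled by the funnel's strength.
; Player movement input inside the tube restores gravity and launches along the view direction; leaving also restores gravity.
; InvertForceDirection flips the force's X component and re-pushes overlapping actors.
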(event OnComponentBeginOverlap(Cylinder)
  (params (OverlappedComponent :type Primitive%20Component%20Object%20Reference) (OtherActor :type Actor%20Object%20Reference) (OtherComp :type Primitive%20Component%20Object%20Reference) (OtherBodyIndex :type Integer) (bFromSweep :type Boolean) (SweepResult :type Hit%20Result%20Structure%20%28by%20ref%29))
  (Development|PrintString "Someone entered the Anti-Gravity Tube!")
  (bind _enabled (Default|IsEnabled (Variables|Default|GetParentFunnel)))
  (if _enabled
    (bind _output_get (Variables|Default|SetActor OtherActor))
    (Utilities|Casting|CastToPortalSuperclass _output_get ; Ignore Portals, otherwise the funnel might try to push e.g. the Portal's arrow.
      (:CastFailed
        (bind _asfirst_person_character (Utilities|Casting|CastToFirstPersonCharacter _output_get)
          (:then
            ;[1 1 1] Actor is FirstPersonCharacter
            (bind _output_get_2 (Variables|Default|SetFirstPersonCharacter _asfirst_person_character))
            (CallFunction|PushFirstPersonCharacter _output_get_2))
          (:CastFailed
            (Development|PrintString "Not FP Character")
            ;[1 1 1] Actor is object
            (CallFunction|PushNonFPSObject (Variables|Default|GetActor))))))))

(event OnComponentEndOverlap(Cylinder)
  (params (OverlappedComponent :type Primitive%20Component%20Object%20Reference) (OtherActor :type Actor%20Object%20Reference) (OtherComp :type Primitive%20Component%20Object%20Reference) (OtherBodyIndex :type Integer))
  (bind _output_get (Variables|Default|SetActor OtherActor))
  (bind _asfirst_person_character (Utilities|Casting|CastToFirstPersonCharacter _output_get)
    (:then
      ;[1 1 1] Drop player
      (CallFunction|ReleasePlayer _asfirst_person_character))
    (:CastFailed
      ;[1 1 1] Drop objects
      (Physics|SetSimulatePhysics (Actor|GetComponentbyClass (Variables|Default|GetActor) "/Script/Engine.PrimitiveComponent") true)
      (Physics|SetEnableGravity (Actor|GetComponentbyClass (Variables|Default|GetActor) "/Script/Engine.PrimitiveComponent") true))))

(event Custom|OnPlayerMovement
  ;[1 1 1] Release Player when he tries to move.
  ;;[1 1 1] Is player currently in Anti-Gravitiy-Tube?
  (if (Utilities|Array|ContainsItem (Collision|GetOverlappingActors 0 :!class /Script/Engine.Actor) (stale EventBeginPlay _asfirst_person_character))
    (CallFunction|ReleasePlayer (stale EventBeginPlay _asfirst_person_character))
    (Character|LaunchCharacter (stale EventBeginPlay _asfirst_person_character) (* (Math|Rotator|GetRotationXVector (Transformation|GetActorRotation (Pawn|GetController (stale EventBeginPlay _asfirst_person_character)))) 1e+02) true true) ; Make player move into the direction he's looking at.
  ))

(event EventBeginPlay
  ;[1 1 1] Release Player when he tries to move.
  (bind _asfirst_person_character (Utilities|Casting|CastToFirstPersonCharacter (Game|Player|GetPlayerPawn 0)))
  (EventDispatchers|BindEventtoPlayerMoving _asfirst_person_character (delegate Custom|OnPlayerMovement)))

(event Collision|EventActorBeginOverlap
  (params (OtherActor :type Actor%20Object%20Reference)))

(event EventTick
  (params (DeltaSeconds :type Float%20%28single-precision%29)))

(fn ConstructionScript)

(fn MoveActortoCenterOfTube
  (params (Actor :type Actor%20Object%20Reference))
  (bind _defaultsceneroot (Variables|Default|GetDefaultSceneRoot))
  (bind _returnvalue (Transformation|GetWorldTransform _defaultsceneroot))
  (Transformation|SetActorLocation Actor (Math|Transform|TransformLocation _returnvalue (Math|Vector|MakeVector (.x (Math|Transform|InverseTransformLocation _returnvalue (Transformation|GetActorLocation Actor))) 0.0 0.0)) false false))

(fn CalculateForceStrength
  (bind _parentfunnel (Variables|Default|GetParentFunnel))
  (return (* (Variables|Default|GetForceDirection) (* (Variables|/Game/Portals/ExcursionFunnel/ExcursionFunnel_BP.ExcursionFunnel_BP_C|GetForceStrength _parentfunnel) (Variables|/Game/Portals/ExcursionFunnel/ExcursionFunnel_BP.ExcursionFunnel_BP_C|GetForceIncreaser _parentfunnel)))))

(fn ReleasePlayer
  (params (Player :type First%20Person%20Character%20Object%20Reference))
  (bind _capsulecomponent (Variables|/Script/Engine.Character|GetCapsuleComponent Player))
  (Physics|SetSimulatePhysics _capsulecomponent false)
  (Physics|SetEnableGravity _capsulecomponent true))

(fn PushFirstPersonCharacter
  (params (Character :type Character%20Object%20Reference))
  (bind _capsulecomponent (Variables|/Script/Engine.Character|GetCapsuleComponent Character))
  (Physics|SetSimulatePhysics _capsulecomponent true)
  (Physics|SetEnableGravity _capsulecomponent false)
  (Physics|SetPhysicsLinearVelocity _capsulecomponent "0, 0, 0" false "None") ; Remove any velocity the player had.
  (CallFunction|MoveActortoCenterOfTube (Variables|Default|GetFirstPersonCharacter))
  (bind _force (CallFunction|CalculateForceStrength))
  (Physics|AddForce _capsulecomponent _force "None" true))

(fn PushNonFPSObject
  (params (Actor :type Actor%20Object%20Reference))
  (bind _returnvalue (Actor|GetComponentbyClass Actor "/Script/Engine.PrimitiveComponent"))
  (bind _returnvalue_2 (Collision|GetCollisionEnabled _returnvalue))
  (if (and (or (Utilities|Enum|Equal(Enum) _returnvalue_2 "PhysicsOnly") (Utilities|Enum|Equal(Enum) _returnvalue_2 "QueryAndPhysics")) (Utilities|Enum|NotEqual(Enum) (Collision|GetCollisionObjectType _returnvalue) "ECC_WorldStatic"))
    (Physics|SetSimulatePhysics _returnvalue true)
    (Physics|SetEnableGravity _returnvalue false)
    (Physics|SetPhysicsLinearVelocity _returnvalue "0, 0, 0" false "None")
    (CallFunction|MoveActortoCenterOfTube (Variables|Default|GetActor))
    (bind _force (CallFunction|CalculateForceStrength))
    (Physics|AddForce _returnvalue _force "None" true)))

(fn InvertForceDirection
  (Variables|Default|SetForceDirection (* (Variables|Default|GetForceDirection) "-1.000000,1.000000,1.000000"))
  (for _array_element (Collision|GetOverlappingActors (Variables|Default|GetCylinder) "/Script/Engine.Actor" :!class /Script/Engine.PrimitiveComponent)
    (Utilities|Casting|CastToPortalSuperclass _array_element ; Ignore Portals, otherwise the funnel might try to push e.g. the Portal's arrow.
      (:CastFailed
        (bind _asfirst_person_character (Utilities|Casting|CastToFirstPersonCharacter _array_element)
          (:then
            (CallFunction|PushFirstPersonCharacter _asfirst_person_character))
          (:CastFailed
            (CallFunction|PushNonFPSObject _array_element)))))))

(fn ReleaseNonFPSObject
  (params (Actor :type Actor%20Object%20Reference))
  (bind _returnvalue (Actor|GetComponentbyClass Actor "/Script/Engine.PrimitiveComponent"))
  (Physics|SetSimulatePhysics _returnvalue true)
  (Physics|SetEnableGravity _returnvalue true)
  (Physics|SetPhysicsLinearVelocity _returnvalue "0, 0, 0" false "None"))