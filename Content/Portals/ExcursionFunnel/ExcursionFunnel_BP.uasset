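; Excursion Funnel emitter that projects a force tube from its base along its arrow, with toggling and force-direction inversion.
; When enabled, it spawns TubeA and line-traces against static objects to stretch it to the hit, or to maximum length.
; It binds to Portal A and player portal events, destroying TubeB when a portal spawns.
; The visibility handler is empty, and nothing here spawns TubeB.
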(event Custom|OnPortalVisibilityChanged
  ;[1 1 1] Bind Event Portal OnSetVisible
)

(event Custom|OnPortalSpawning
  (bind _tubeb (Variables|Default|GetTubeB))
  ;[1 1 1] Remove TubeB if Portal location is changing.
  (Utilities|IsValid _tubeb
    (:Is%20Valid
      (Development|PrintString "Removing Tube B" true true "(R=0.170000,G=0.100721,B=1.000000,A=1.000000)")
      (Collision|SetCollisionEnabled (Variables|/Game/Portals/ExcursionFunnel/ExcursionFunnelTube_BP.ExcursionFunnelTube_BP_C|GetCylinder _tubeb) "NoCollision")
      (Rendering|SetVisibility (Variables|/Script/Engine.Actor|GetRootComponent _tubeb) false true)
      (Actor|DestroyActor (Variables|Default|GetTubeB)))))

(event EventBeginPlay
  (if (Variables|Default|GetEnabled)
    (CallFunction|SpawnTubeA)
    (bind _returnvalue (Actor|GetActorOfClass "/Game/Portals/Portals/Portal_A_BP_Child.Portal_A_BP_Child_C"))
    (Utilities|IsValid _returnvalue
      (:Is%20Valid
        (bind _output_get (Variables|Default|SetPortalA _returnvalue))
        ;[1 1 1] Bind Event Portal OnSetVisible
        (EventDispatchers|BindEventtoOnSetVisible _output_get (delegate Custom|OnPortalVisibilityChanged))
        ;[1 1 1] Bind Event Portal OnPortalSpawning
        (bind _asfirst_person_character (Utilities|Casting|CastToFirstPersonCharacter (Game|GetPlayerCharacter 0)))
        (EventDispatchers|BindEventtoPortalSpawning _asfirst_person_character (delegate Custom|OnPortalSpawning)))
      (:Is%20Not%20Valid
        (Development|PrintString "ERROR! [Excursion Funnel - BeingPlay] Could not find Portal A in level." true true "(R=1.000000,G=0.000000,B=0.059606,A=1.000000)")))))

(event Collision|EventActorBeginOverlap
  (params (OtherActor :type Actor%20Object%20Reference)))

(event EventTick
  (params (DeltaSeconds :type Float%20%28single-precision%29)))

(fn ConstructionScript)

(fn DReleasePlayer
  (params (Player :type First%20Person%20Character%20Object%20Reference))
  (bind _capsulecomponent (Variables|/Script/Engine.Character|GetCapsuleComponent Player))
  (Physics|SetSimulatePhysics _capsulecomponent false)
  (Physics|SetEnableGravity _capsulecomponent true))

(fn DMoveActortoCenterOfTube
  (params (Actor :type Actor%20Object%20Reference))
  (bind _defaultsceneroot (Variables|Default|GetDefaultSceneRoot))
  (bind _returnvalue (Transformation|GetWorldTransform _defaultsceneroot))
  (Transformation|SetActorLocation Actor (Math|Transform|TransformLocation _returnvalue (Math|Vector|MakeVector (.x (Math|Transform|InverseTransformLocation _returnvalue (Transformation|GetActorLocation Actor))) 0.0 0.0)) false false))

(fn DCalculateForceDirectionandStrength
  (return (* (Math|Vector|GetForwardVector (Variables|Default|GetArrow self)) (* (Variables|Default|GetForceStrength) (Variables|Default|GetForceIncreaser)))))

(fn SetTubeTransform
  (params (Tube :type Excursion%20Funnel%20Tube%20BP%20Object%20Reference) (StartLocation :type Vector) (TraceDirection :type Vector))
  (LocalVariables|SetTubeVar Tube)
  (LocalVariables|SetStartLocationVar StartLocation)
  (LocalVariables|SetTraceDirectionVar TraceDirection)
  ;[1 1 1] Find first static object / wall the tube hits.
  (bind (_outhit _returnvalue) (Collision|LineTraceForObjects (LocalVariables|GetStartLocationVar) (+ (LocalVariables|GetStartLocationVar) (* (LocalVariables|GetTraceDirectionVar) (LocalVariables|GetLineTraceLength))) (Utilities|Array|MakeArray "ObjectTypeQuery1") false 0 "None"))
  (if _returnvalue
    ;[1 1 1] Line trace hit wall. Calculate bridge length and position.
    (LocalVariables|SetScalingFactorZ (/ (.Distance (Collision|BreakHitResult _outhit)) (LocalVariables|GetDistanceToScaleConversionValue)))
    (Transformation|SetActorLocationAndRotation (LocalVariables|GetTubeVar) (+ (LocalVariables|GetStartLocationVar) (/ (- (.Location (Collision|BreakHitResult _outhit)) (LocalVariables|GetStartLocationVar)) 2)) (Math|Rotator|MakeRotator (.roll (Transformation|GetActorRotation)) (.pitch (Math|Conversions|RotationFromXVector (LocalVariables|GetTraceDirectionVar))) (.yaw (Math|Conversions|RotationFromXVector (LocalVariables|GetTraceDirectionVar)))))
    (Transformation|SetActorRelativeScale3D (LocalVariables|GetTubeVar) (Math|Vector|MakeVector 1.0 1.0 (LocalVariables|GetScalingFactorZ)))
    (else
      ;[1 1 1] Line trace didn't hit anything. Extend tube to maximum length.
      (LocalVariables|SetScalingFactorZ (/ (Variables|Default|GetMaxTubeLength) (LocalVariables|GetDistanceToScaleConversionValue)))
      (Transformation|SetActorLocationAndRotation (LocalVariables|GetTubeVar) (+ (LocalVariables|GetStartLocationVar) (* TraceDirection (/ (Variables|Default|GetMaxTubeLength) 2.0))) (Math|Rotator|MakeRotator (.roll (Transformation|GetActorRotation)) (.pitch (Math|Conversions|RotationFromXVector (LocalVariables|GetTraceDirectionVar))) (.yaw (Math|Conversions|RotationFromXVector (LocalVariables|GetTraceDirectionVar)))))
      (Transformation|SetActorRelativeScale3D (LocalVariables|GetTubeVar) (Math|Vector|MakeVector 1.0 1.0 (LocalVariables|GetScalingFactorZ))))))

(fn SpawnTubeA
  (bind _returnvalue (Game|SpawnActorfromClass "/Game/Portals/ExcursionFunnel/ExcursionFunnelTube_BP.ExcursionFunnelTube_BP_C" (Math|Transform|MakeTransform "0, 0, 0" (Transformation|GetActorRotation) "1,1,1") "Undefined" 0 self (Math|Vector|GetForwardVector (Variables|Default|GetArrow)) 0))
  (bind _output_get (Variables|Default|SetTubeA _returnvalue))
  (CallFunction|SetTubeTransform _output_get (Transformation|GetWorldLocation (Variables|Default|GetBase)) (Math|Vector|GetForwardVector (Variables|Default|GetArrow))))

(fn SetEnabled
  (params (Enabled :type Boolean))
  (bind _tubea (Variables|Default|GetTubeA))
  (bind _tubeb (Variables|Default|GetTubeB))
  (Variables|Default|SetEnabled Enabled)
  (if Enabled
    (CallFunction|SpawnTubeA)
    (else
      (Utilities|FlowControl|Sequence
        (:then_0
          (Utilities|IsValid _tubea
            (:Is%20Valid
              (Actor|DestroyActor _tubea))))
        (:then_1
          (Utilities|IsValid _tubeb
            (:Is%20Valid
              (Actor|DestroyActor _tubeb))))))))

(fn IsEnabled
  (return (Variables|Default|GetEnabled)))

(fn InvertForceDirectionOfTubes
  (bind _tubeb (Variables|Default|GetTubeB))
  (bind _tubea (Variables|Default|GetTubeA))
  (bind _enabled (CallFunction|IsEnabled))
  (if _enabled
    (Utilities|IsValid _tubea
      (:Is%20Valid
        (Default|InvertForceDirection _tubea)
        (Utilities|IsValid _tubeb
          (:Is%20Valid
            (Default|InvertForceDirection _tubeb)))))
    (else
      (Development|PrintString "NOTE NABLED"))))