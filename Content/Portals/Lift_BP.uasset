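; Moving lift platform that travels between StartPoint and EndPoint, optionally triggered by the first-person character stepping on or off its box.
; A timeline lerps the platform's location, with MovementSpeed as play rate, returning after WaitTime and disabling itself back at the start.
; SetEnabled stops the timeline or plays it when the remembered direction is forward.
; The construction script places a game-hidden destination preview at EndPoint.
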(event OnComponentBeginOverlap(Box)
  (params (OverlappedComponent :type Primitive%20Component%20Object%20Reference) (OtherActor :type Actor%20Object%20Reference) (OtherComp :type Primitive%20Component%20Object%20Reference) (OtherBodyIndex :type Integer) (bFromSweep :type Boolean) (SweepResult :type Hit%20Result%20Structure%20%28by%20ref%29))
  ;[1 1 1] Player stepped on platform
  (if (Variables|Default|GetMoveWhenPlayerSteppedOn)
    (Utilities|Casting|CastToFirstPersonCharacter OtherActor)
    (if (Variables|Default|GetEnabled)
      (Audio|Components|Audio|Play (Variables|Default|GetTimeline_0)))))

(event OnComponentEndOverlap(Box)
  (params (OverlappedComponent :type Primitive%20Component%20Object%20Reference) (OtherActor :type Actor%20Object%20Reference) (OtherComp :type Primitive%20Component%20Object%20Reference) (OtherBodyIndex :type Integer))
  ;[1 1 1] Player left platform
  (if (Variables|Default|GetMoveWhenPlayerSteppedOn)
    (Utilities|Casting|CastToFirstPersonCharacter OtherActor)
    (Utilities|String|Reverse (Variables|Default|GetTimeline_0))))

(event EventBeginPlay
  ;[1 1 1] Position platform at StartPoint
  (Transformation|SetRelativeLocation (Variables|Default|GetLift) (Variables|Default|GetStartPoint) false false)
  ;[1 1 1] Apply movementSpeed by setting the PlayRate of the Timeline
  (Components|Timeline|SetPlayRate (Variables|Default|GetTimeline_0) (Variables|Default|GetMovementSpeed)))

(event Collision|EventActorBeginOverlap
  (params (OtherActor :type Actor%20Object%20Reference)))

(event EventTick
  (params (DeltaSeconds :type Float%20%28single-precision%29)))

(fn ConstructionScript
  ;[1 1 1] Needs to be set here. Once I defined a constructor for this object, the "Hidden In Game" option in the "Details" panel doesn't work anymore.
  (Development|SetHiddeninGame (Variables|Default|GetDestinationPreview) true true)
  (Transformation|SetRelativeLocation (Variables|Default|GetDestinationPreview) (Variables|Default|GetEndPoint) false false))

(fn SetEnabled
  (params (Enabled :type Boolean))
  (bind _timeline_0 (Variables|Default|GetTimeline_0))
  (bind _output_get (Variables|Default|SetEnabled Enabled))
  (if _output_get
    (if (Utilities|Enum|Equal(Enum) (Variables|Default|GetMemoDirection) "Forward")
      (Audio|Components|Audio|Play _timeline_0))
    (else
      (Audio|Components|Audio|Stop _timeline_0))))