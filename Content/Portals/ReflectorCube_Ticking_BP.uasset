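; Laser reflector cube that keeps the laser emitter hitting it up to date as the cube moves.
; Tick, throttled to a 0.01-second interval, compares the actor location to the last stored one within a small tolerance.
; On a change it calls UpdateLasers on HittingLaserEmitter and stores the new location, clearing the Update flag during the call as a guard.
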(event EventBeginPlay
  (Actor|Tick|SetActorTickInterval 0.01))

(event Collision|EventActorBeginOverlap
  (params (OtherActor :type Actor%20Object%20Reference)))

(event EventTick
  (params (DeltaSeconds :type Float%20%28single-precision%29))
  (if (Variables|Default|GetUpdate)
    (if (Math|Vector|NotEqual(Vector) (Variables|Default|GetOldLocation) (Transformation|GetActorLocation) 0.001)
      (Variables|Default|SetUpdate false)
      (Default|UpdateLasers (Variables|Default|GetHittingLaserEmitter))
      (Variables|Default|SetOldLocation (Transformation|GetActorLocation))
      (Variables|Default|SetUpdate true))))

(fn ConstructionScript)