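; Energy ball actor from the Portals game's ball source, which removes itself by age or on impact.
; When Lifespan is positive, a looping one-second timer counts and prints SecondsAlive, destroying the ball once the count reaches Lifespan.
; With DestroyOnFirstHit set, a Sphere hit on anything other than BallTarget also destroys it.
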(event OnComponentHit(Sphere)
  (params (HitComponent :type Primitive%20Component%20Object%20Reference) (OtherActor :type Actor%20Object%20Reference) (OtherComp :type Primitive%20Component%20Object%20Reference) (NormalImpulse :type Vector :default "0, 0, 0") (Hit :type Hit%20Result%20Structure%20%28by%20ref%29))
  ;[1 1 1] Destroy on first hit
  (if (and (Variables|Default|GetDestroyOnFirstHit) (not (== OtherActor (Variables|Default|GetBallTarget))))
    (Actor|DestroyActor)))

(event Custom|OnSecondElapsed
  ;[1 1 1] Destroy if lifespan has been exceeded.
  (if (>= (Variables|Default|GetSecondsAlive) (Variables|Default|GetLifespan))
    (Actor|DestroyActor)
    (else
      (bind _result (Math|Integer|IncrementInt (Variables|Default|GetSecondsAlive))
        (:%20%20
          (bind _output_get (Variables|Default|SetSecondsAlive _result))
          (Development|PrintString (Utilities|String|ToString(Integer) _output_get)))))))

(event EventBeginPlay
  (if (> (Variables|Default|GetLifespan) 0)
    (Utilities|Time|SetTimerbyEvent (delegate Custom|OnSecondElapsed) 1.0 true)))

(event Collision|EventActorBeginOverlap
  (params (OtherActor :type Actor%20Object%20Reference)))

(event EventTick
  (params (DeltaSeconds :type Float%20%28single-precision%29)))

(fn ConstructionScript)