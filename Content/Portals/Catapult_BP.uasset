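; Catapult pad that launches the player or other actors overlapping its collision box while enabled.
; Players get LaunchCharacter with an adjusted power, intended to match object distance; other actors get a velocity-change impulse on their primitive component.
; A helper pitches the local-space forward vector by Angle and scales it by boosted jump power, without converting back to world space.
; A shared cooldown gates repeat launches.
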(event OnComponentBeginOverlap(CollisionBox)
  (params (OverlappedComponent :type Primitive%20Component%20Object%20Reference) (OtherActor :type Actor%20Object%20Reference) (OtherComp :type Primitive%20Component%20Object%20Reference) (OtherBodyIndex :type Integer) (bFromSweep :type Boolean) (SweepResult :type Hit%20Result%20Structure%20%28by%20ref%29))
  (if (Variables|Default|GetEnabled)
    (if (Utilities|ClassIsChildOf (Utilities|GetClass OtherActor) "/Game/FirstPersonCPP/Blueprints/FirstPersonCharacter.FirstPersonCharacter_C")
      ;[1 1 1] Catapult Player
      (bind _asfirst_person_character (Utilities|Casting|CastToFirstPersonCharacter OtherActor)
        (:then
          (if (Variables|Default|GetCanCatapult)
            (Variables|Default|SetCanCatapult false)
            (bind _velocityvector (CallFunction|CalculateLaunchVelocityVector (* (Variables|Default|GetJumpPower) (Variables|Default|GetPlayerJumpPowerAdjustment))))
            (Character|LaunchCharacter _asfirst_person_character _velocityvector true true)
            (Utilities|FlowControl|Delay (Variables|Default|GetCooldown))
            (Variables|Default|SetCanCatapult true)))
        (:CastFailed
          (Development|PrintString "Cast failed")))
      (else
        ;[1 1 1] Catapult object
        (if (Variables|Default|GetCanCatapult)
          (Variables|Default|SetCanCatapult false)
          (bind _velocityvector_2 (CallFunction|CalculateLaunchVelocityVector (Variables|Default|GetJumpPower)))
          (Physics|AddImpulse (Actor|GetComponentbyClass OtherActor "/Script/Engine.PrimitiveComponent") _velocityvector_2 "None" true)
          (Utilities|FlowControl|Delay (Variables|Default|GetCooldown))
          (Variables|Default|SetCanCatapult true))))))

(event EventBeginPlay)

(event Collision|EventActorBeginOverlap
  (params (OtherActor :type Actor%20Object%20Reference)))

(event EventTick
  (params (DeltaSeconds :type Float%20%28single-precision%29)))

(fn ConstructionScript)

(fn CalculateLaunchVelocityVector
  (params (JumpPower :type Float%20%28single-precision%29))
  (return (* (Math|Vector|RotateVector (Math|Transform|InverseTransformDirection (Transformation|GetActorTransform) (Transformation|GetActorForwardVector)) (Math|Rotator|MakeRotator 0.0 (Variables|Default|GetAngle) 0.0)) (* JumpPower (LocalVariables|GetJumpPowerIncreaser)))))