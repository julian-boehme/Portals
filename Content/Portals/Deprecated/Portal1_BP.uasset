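; Deprecated portal actor that teleports the first-person player and objects overlapping its mesh to a linked Portal2.
; Overlap logic separates player, held object and loose object, disabling Portal2 for a delay to prevent bounce-back.
; Players snap to the destination arrow, while objects keep their portal-relative offset with velocity rotated by the exit's rotation.
; Held objects are briefly released, teleported, regrabbed and repositioned at their rotated offset from the player.
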(event OnComponentBeginOverlap(PortalMesh)
  (params (OverlappedComponent :type Primitive%20Component%20Object%20Reference) (OtherActor :type Actor%20Object%20Reference) (OtherComp :type Primitive%20Component%20Object%20Reference) (OtherBodyIndex :type Integer) (bFromSweep :type Boolean) (SweepResult :type Hit%20Result%20Structure%20%28by%20ref%29))
  (bind _returnvalue (Game|GetPlayerCharacter 0))
  (bind _returnvalue_2 (Actor|GetComponentbyClass _returnvalue "/Script/Portals.FPGrabber"))
  (bind _grabbedobject (Variables|/Script/Portals.FPGrabber|GetGrabbedObject _returnvalue_2))
  (Utilities|IsValid (Variables|Default|GetPortal2)
    (:Is%20Valid
      (if (Variables|Default|GetCanTeleport)
        (Variables|/Game/Portals/Deprecated/Portal2_BP.Portal2_BP_C|SetCanTeleport (Variables|Default|GetPortal2) false)
        ;[1 1 1] Is actor player or object?
        (if (Utilities|ClassIsChildOf (Utilities|GetClass OtherActor) "/Game/FirstPersonCPP/Blueprints/FirstPersonCharacter.FirstPersonCharacter_C")
          ;[1 1 1] Is Player holding object?
          (if (Utilities|IsValid _grabbedobject)
            ;[1 1 1] Teleport player holding object
            (bind _asfirst_person_character (Utilities|Casting|CastToFirstPersonCharacter OtherActor))
            (CallFunction|TeleportPlayerHoldingObject _asfirst_person_character _grabbedobject self (Variables|Default|GetPortal2))
            ;[1 1 1] Cleanup
            (Utilities|FlowControl|Delay (Variables|Default|GetTeleportationDelay) :!label _label)
            (Variables|/Game/Portals/Deprecated/Portal2_BP.Portal2_BP_C|SetCanTeleport (Variables|Default|GetPortal2) true)
            (else
              ;[1 1 1] Teleport player not holding object
              (bind _asfirst_person_character_2 (Utilities|Casting|CastToFirstPersonCharacter OtherActor)
                (:then
                  (CallFunction|TeleportPlayer _asfirst_person_character_2 self (Variables|Default|GetPortal2))
                  (goto _label))
                (:CastFailed
                  (Development|PrintString "FPSCharacter Cast FAILED!")))))
          (else
            ;[1 1 1] Is object held by player?
            (if (== OtherActor (Variables|/Script/Portals.FPGrabber|GetGrabbedObject (Actor|GetComponentbyClass (Game|GetPlayerCharacter 0) "/Script/Portals.FPGrabber")))
              ;[1 1 1] Teleport player holding object
              (bind _asfirst_person_character_3 (Utilities|Casting|CastToFirstPersonCharacter (Game|GetPlayerCharacter 0)))
              (CallFunction|TeleportPlayerHoldingObject _asfirst_person_character_3 OtherActor self (Variables|Default|GetPortal2))
              (goto _label)
              (else
                ;[1 1 1] If object not held by player. teleport object, else wait until player is teleported
                (CallFunction|TeleportObject OtherActor self (Variables|Default|GetPortal2))
                (goto _label)))))))
    (:Is%20Not%20Valid
      (Development|PrintString "ERROR! Portal 2 variable is not set on Portal 1" true true "(R=1.000000,G=0.000000,B=0.078800,A=1.000000)"))))

(event EventBeginPlay)

(event Collision|EventActorBeginOverlap
  (params (OtherActor :type Actor%20Object%20Reference)))

(event EventTick
  (params (DeltaSeconds :type Float%20%28single-precision%29)))

(fn ConstructionScript)

(fn TeleportObject
  (params (Actor :type Actor%20Object%20Reference) (SrcPortal :type Actor%20Object%20Reference) (DestPortal :type Actor%20Object%20Reference))
  (bind _locatdestportal (CallFunction|GetOffsetfromObjtoPortal Actor SrcPortal DestPortal))
  ;[1 1 1] Transform object
  (Transformation|SetActorTransform Actor _locatdestportal false true)
  ;[1 1 1] Change velocity direction to dest portal direction
  (Physics|SetPhysicsLinearVelocity (Actor|GetComponentbyClass Actor "/Script/Engine.PrimitiveComponent") (Math|Vector|RotateVector (Transformation|GetVelocity Actor) (.rotation (Transformation|GetActorTransform DestPortal))) false "None"))

(fn TeleportPlayer
  (params (Player :type First%20Person%20Character%20Object%20Reference) (SrcPortal :type Portal%201%20BP%20Object%20Reference) (DestPortal :type Portal%202%20BP%20Object%20Reference))
  (bind _arrow (Variables|/Game/Portals/Deprecated/Portal2_BP.Portal2_BP_C|GetArrow DestPortal))
  (bind _returnvalue (Transformation|GetWorldTransform _arrow))
  (Pawn|SetControlRotation (Pawn|GetController Player) (.rotation _returnvalue))
  (Transformation|SetActorLocation Player (.location _returnvalue) false true))

(fn TeleportPlayerHoldingObject
  (params (Player :type First%20Person%20Character%20Object%20Reference) (HeldObject :type Actor%20Object%20Reference) (SrcPortal :type Portal%201%20BP%20Object%20Reference) (DestPortal :type Portal%202%20BP%20Object%20Reference))
  (bind _returnvalue (Actor|GetComponentbyClass Player "/Script/Portals.FPGrabber"))
  (bind _output_get (LocalVariables|SetOldObjectLocation (Transformation|GetActorLocation HeldObject)))
  (bind _output_get_2 (LocalVariables|SetOldPlayerLocation (Transformation|GetActorLocation Player)))
  (bind _output_get_3 (LocalVariables|SetObjectOffsetFromPlayer (- _output_get _output_get_2)))
  (CallFunction|TeleportPlayer Player SrcPortal DestPortal)
  ;[1 1 1] Teleport object with offset from player, otherwise object and player will be teleported to the same location, which results in the player being pushed down into the ground be the object.
  (Class|FPGrabber|ReleaseTemporarily _returnvalue)
  (CallFunction|TeleportObject HeldObject SrcPortal DestPortal)
  (Class|FPGrabber|GrabAfterTemporaryRelease _returnvalue)
  ;;[1 1 1] Re-apply object's offset after teleporting
  (Transformation|SetActorLocation HeldObject (+ (Transformation|GetActorLocation Player) (Math|Vector|RotateVector _output_get_3 (Transformation|GetActorRotation DestPortal))) false true))

(fn GetOffsetfromObjtoPortal
  (params (Actor :type Actor%20Object%20Reference) (SrcPortal :type Actor%20Object%20Reference) (DestPortal :type Actor%20Object%20Reference))
  (bind _returnvalue (Transformation|GetActorTransform Actor))
  (return (Math|Transform|MakeTransform (+ (Math|Vector|RotateVector (- (.location _returnvalue) (Transformation|GetActorLocation SrcPortal)) (Transformation|GetActorRotation DestPortal)) (Transformation|GetActorLocation DestPortal)) (Transformation|GetActorRotation DestPortal) (.scale _returnvalue))))