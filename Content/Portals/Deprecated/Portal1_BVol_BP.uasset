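; Portal actor, in a deprecated folder, that teleports the first-person character and objects to a linked Portal2.
; Objects entering the front box get a SmallCube stand-in at Portal2, tracked in a map and repositioned every Tick by rotated relative offset.
; Passing into the back box moves the original onto its copy, waiting for FPGrabber release if held, or following the player's teleport.
; CanTeleport flags guard against bouncing back; debug prints remain.
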(event OnComponentEndOverlap(FrontCollisionBox)
  (params (OverlappedComponent :type Primitive%20Component%20Object%20Reference) (OtherActor :type Actor%20Object%20Reference) (OtherComp :type Primitive%20Component%20Object%20Reference) (OtherBodyIndex :type Integer))
  (bind _objectsmapping (Variables|Default|GetObjectsMapping))
  ;[1 1 1] Is object in back collision box
  (if (Utilities|Array|ContainsItem (Collision|GetOverlappingActors (Variables|Default|GetBackCollisionBox) 0 :!class /Script/Engine.PrimitiveComponent) OtherActor)
    ;[1 1 1] Is object currently held by player? If so, do nothing (until released), otherwise teleport.
    (if (not (== (Variables|/Script/Portals.FPGrabber|GetGrabbedObject (Actor|GetComponentbyClass (Game|GetPlayerCharacter 0) "/Script/Portals.FPGrabber")) OtherActor))
      (CallFunction|ReplaceDuplicatewithOriginal OtherActor))
    (else
      ;[1 1 1] Removes objects that leave the front collision box (but not through the portal), from the objectsArray and destroys the copies
      (if (Utilities|Map|Contains _objectsmapping OtherActor)
        (Actor|DestroyActor (.Value (Utilities|Map|Find _objectsmapping OtherActor)))
        (bind _returnvalue (Utilities|Map|Remove _objectsmapping OtherActor))
        (if (not _returnvalue)
          (Development|PrintString "Error! Could not delete object from objectArray after leaving front collision box!" true true "(R=1.000000,G=0.000000,B=0.046319,A=1.000000)"))))))

(event OnComponentBeginOverlap(FrontCollisionBox)
  (params (OverlappedComponent :type Primitive%20Component%20Object%20Reference) (OtherActor :type Actor%20Object%20Reference) (OtherComp :type Primitive%20Component%20Object%20Reference) (OtherBodyIndex :type Integer) (bFromSweep :type Boolean) (SweepResult :type Hit%20Result%20Structure%20%28by%20ref%29))
  (bind _portal2 (Variables|Default|GetPortal2))
  (bind _defaultsceneroot (Variables|/Game/Portals/Deprecated/Portal2_BVol_BP.Portal2_BVol_BP_C|GetDefaultSceneRoot _portal2))
  ;[1 1 1] Duplicate objects entering FrontCollisionBox
  (if (not (Utilities|ClassIsChildOf (Utilities|GetClass OtherActor) "/Game/FirstPersonCPP/Blueprints/FirstPersonCharacter.FirstPersonCharacter_C"))
    (CallFunction|DuplicateObject OtherActor (Transformation|GetWorldLocation (Variables|Default|GetDefaultSceneRoot)) (Transformation|GetWorldLocation _defaultsceneroot) (Transformation|GetWorldRotation _defaultsceneroot))))

(event OnComponentBeginOverlap(BackCollisionBox)
  (params (OverlappedComponent :type Primitive%20Component%20Object%20Reference) (OtherActor :type Actor%20Object%20Reference) (OtherComp :type Primitive%20Component%20Object%20Reference) (OtherBodyIndex :type Integer) (bFromSweep :type Boolean) (SweepResult :type Hit%20Result%20Structure%20%28by%20ref%29))
  (bind _returnvalue (Game|GetPlayerCharacter 0))
  (bind _portal2 (Variables|Default|GetPortal2))
  (bind _returnvalue_2 (Actor|GetComponentbyClass _returnvalue "/Script/Portals.FPGrabber"))
  (bind _grabbedobject (Variables|/Script/Portals.FPGrabber|GetGrabbedObject _returnvalue_2))
  ;[1 1 1] Teleport Player
  (if (Utilities|ClassIsChildOf (Utilities|GetClass OtherActor) "/Game/FirstPersonCPP/Blueprints/FirstPersonCharacter.FirstPersonCharacter_C")
    (if (Variables|Default|GetCanTeleport)
      (Variables|/Game/Portals/Deprecated/Portal2_BVol_BP.Portal2_BVol_BP_C|SetCanTeleport (Variables|Default|GetPortal2) false)
      (bind _asfirst_person_character (Utilities|Casting|CastToFirstPersonCharacter OtherActor))
      (Development|PrintString "Is FP Character")
      (Pawn|SetControlRotation (Pawn|GetController _asfirst_person_character) (Transformation|GetActorRotation _portal2))
      (Transformation|SetActorLocation _asfirst_person_character (Transformation|GetActorLocation _portal2) false false)
      ;;[1 1 1] Is Player holding object?
      (if (Utilities|IsValid _grabbedobject)
        (CallFunction|ReplaceDuplicatewithOriginal _grabbedobject) ; Teleport held object
        (Utilities|FlowControl|Delay 0.2)
        (Variables|/Game/Portals/Deprecated/Portal2_BVol_BP.Portal2_BVol_BP_C|SetCanTeleport (Variables|Default|GetPortal2) true)
        (else
          (Utilities|FlowControl|Delay 0.2)
          (Variables|/Game/Portals/Deprecated/Portal2_BVol_BP.Portal2_BVol_BP_C|SetCanTeleport (Variables|Default|GetPortal2) true))))))

(event Custom|OnRelease_Event_0
  ;[1 1 1] Bind FPGrabber OnRelease Event
  ;;[1 1 1] If released object is in Back Collision Box, teleport.
  (if (Utilities|Array|ContainsItem (Collision|GetOverlappingActors (Variables|Default|GetBackCollisionBox) 0 :!class /Script/Engine.PrimitiveComponent) 0)
    (CallFunction|ReplaceDuplicatewithOriginal (Variables|/Script/Portals.FPGrabber|GetGrabbedObject (Actor|GetComponentbyClass (Game|GetPlayerCharacter 0) "/Script/Portals.FPGrabber")))
    (Development|PrintString "Released Grabbed Object")))

(event EventBeginPlay
  (bind _returnvalue (Game|GetPlayerCharacter 0))
  (bind _returnvalue_2 (Actor|GetComponentbyClass _returnvalue "/Script/Portals.FPGrabber"))
  ;[1 1 1] BeginPlay Event
  ;[1 1 1] Bind FPGrabber OnRelease Event
  (if (Utilities|IsValid _returnvalue_2)
    (EventDispatchers|AssignOnRelease _returnvalue_2 (delegate Custom|OnRelease_Event_0))
    (else
      (Development|PrintString "FPGrabber not valid!"))))

(event EventTick
  (params (DeltaSeconds :type Float%20%28single-precision%29))
  ;[1 1 1] Upate objects locations in dest portal.
  (CallFunction|UpdateObjectsLocations))

(fn ConstructionScript)

(fn DuplicateObject
  (params (SrcActor :type Actor%20Object%20Reference) (SourceLocation :type Vector) (DestinatinLocation :type Vector) (DestinationRotation :type Rotator))
  (bind _objectsmapping (Variables|Default|GetObjectsMapping))
  (bind _portal2 (Variables|Default|GetPortal2))
  ;[1 1 1] Is object already in objectsMapping?
  (if (Utilities|Map|Contains _objectsmapping SrcActor)
    (Development|PrintString "Does contain object")
    (else
      ;[1 1 1] Debugging
      (Development|PrintString (Utilities|String|Append (Utilities|GetDisplayName SrcActor) " Entered"))
      ;[1 1 1] Create copy of object at dest portal.
      (bind _returnvalue (Game|SpawnActorfromClass "/Game/Portals/Debugging/SmallCube.SmallCube_C" (Math|Transform|MakeTransform (+ (Math|Vector|RotateVector (- (Transformation|GetActorLocation SrcActor) SourceLocation) (Transformation|GetActorRotation _portal2)) (Transformation|GetActorLocation _portal2))) "AlwaysSpawn" (Components|GetOwner SrcActor) (Game|GetInstigator SrcActor)))
      (Development|PrintString (Utilities|GetClassDisplayName (Utilities|GetClass SrcActor)))
      (Utilities|Map|Add _objectsmapping SrcActor _returnvalue)
      (return))))

(fn UpdateObjectsLocations
  (bind _objectsmapping (Variables|Default|GetObjectsMapping))
  (bind _portal2 (Variables|Default|GetPortal2))
  ;[1 1 1] Foreach object in Collision Box, find matching object on the other portal.
  (bind _keys (Utilities|Map|Keys _objectsmapping))
  (for _array_element _keys
    (if (.ReturnValue (Utilities|Map|Find _objectsmapping _array_element))
      (Transformation|SetActorLocationAndRotation (.Value (Utilities|Map|Find _objectsmapping _array_element)) (+ (Math|Vector|RotateVector (- (Transformation|GetActorLocation _array_element) (Transformation|GetActorLocation)) (Transformation|GetActorRotation _portal2)) (Transformation|GetActorLocation _portal2)) (Transformation|GetActorRotation _array_element)))))

(fn ReplaceDuplicatewithOriginal
  (params (Actor :type Actor%20Object%20Reference))
  (bind _objectsmapping (Variables|Default|GetObjectsMapping))
  (bind (_value _returnvalue) (Utilities|Map|Find _objectsmapping Actor))
  (bind _returnvalue_2 (Transformation|GetActorTransform _value))
  ;[1 1 1] Object went throug portal: Move original object to copy location. Destroy copy and remove entry in ObjectsMapping.
  (if (Variables|Default|GetCanTeleport)
    (Variables|/Game/Portals/Deprecated/Portal2_BVol_BP.Portal2_BVol_BP_C|SetCanTeleport (Variables|Default|GetPortal2) false)
    (if (Utilities|Map|Contains _objectsmapping Actor)
      (if _returnvalue
        (Transformation|SetActorTransform Actor (Math|Transform|MakeTransform (.location _returnvalue_2) (.rotation _returnvalue_2) "1,1,1"))
        (Actor|DestroyActor _value)
        (bind _returnvalue_3 (Utilities|Map|Remove _objectsmapping Actor))
        (if _returnvalue_3
          _)))))