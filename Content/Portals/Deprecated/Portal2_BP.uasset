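; Deprecated second portal of a linked pair, built to send the player and physics objects to Portal1; its teleport logic is disconnected from the overlap event.
; That logic moves the player with any held object, using temporary grabber release, and locks Portal1 against re-triggering until a delay ends.
; TeleportObject rotates an object's portal-relative offset and velocity by the destination's rotation, keeping the object's own rotation and scale.
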(event OnComponentBeginOverlap(PortalMesh)
  (params (OverlappedComponent :type Primitive%20Component%20Object%20Reference) (OtherActor :type Actor%20Object%20Reference) (OtherComp :type Primitive%20Component%20Object%20Reference) (OtherBodyIndex :type Integer) (bFromSweep :type Boolean) (SweepResult :type Hit%20Result%20Structure%20%28by%20ref%29)))

(event EventBeginPlay)

(event Collision|EventActorBeginOverlap
  (params (OtherActor :type Actor%20Object%20Reference)))

(event EventTick
  (params (DeltaSeconds :type Float%20%28single-precision%29)))

(fn ConstructionScript)

(fn TeleportObject
  (params (Actor :type Actor%20Object%20Reference) (SrcPortal :type Actor%20Object%20Reference) (DestPortal :type Actor%20Object%20Reference))
  (bind _returnvalue (Transformation|GetActorTransform DestPortal))
  (bind _returnvalue_2 (Transformation|GetActorTransform Actor))
  ;[1 1 1] Transform object
  (Transformation|SetActorTransform Actor (Math|Transform|MakeTransform (+ (Math|Vector|RotateVector (- (Transformation|GetActorLocation Actor) (.location (Transformation|GetActorTransform SrcPortal))) (.rotation _returnvalue)) (.location _returnvalue)) (.rotation _returnvalue_2) (.scale _returnvalue_2)) false true)
  ;[1 1 1] Change velocity direction to dest portal direction
  (Physics|SetPhysicsLinearVelocity (Actor|GetComponentbyClass Actor "/Script/Engine.PrimitiveComponent") (Math|Vector|RotateVector (Transformation|GetVelocity Actor) (.rotation _returnvalue)) false "None"))

(fn IsFirstPersonCharacter
  (params (Actor :type Actor%20Object%20Reference))
  (return (Utilities|ClassIsChildOf (Utilities|GetClass Actor) "/Game/FirstPersonCPP/Blueprints/FirstPersonCharacter.FirstPersonCharacter_C")))