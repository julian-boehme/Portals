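; Grabber component that lets the first-person player carry physics objects through the owner's PhysicsHandle.
; Each tick it moves the held object to a point at Reach along the camera's forward vector, yawing ReflectiveCubes away from the player so their lasers shoot outward.
; Grab takes the object from its caller and memorizes the grab parameters, allowing a temporary release and re-grab.
; A helper line-traces for physics bodies within reach, while input setup is left unwired.
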(event EventBeginPlay
  (CallFunction|SetupInputComponent)
  (CallFunction|FindPhysicsHandleComponent))

(event EventTick
  (params (DeltaSeconds :type Float%20%28single-precision%29))
  (bind _physicshandle (Variables|Default|GetPhysicsHandle))
  (bind _grabbedobjectvar (Variables|Default|GetGrabbedObjectVar))
  (Utilities|IsValid _physicshandle
    (:Is%20Valid
      (Utilities|IsValid (Class|PhysicsHandleComponent|GetGrabbedComponent _physicshandle)
        (:Is%20Valid
          (bind _end (CallFunction|GetReachLineEnd))
          (Physics|Components|PhysicsHandle|SetTargetLocation _physicshandle _end)
          ;[1 1 1] Keep rotation of ReflectorCubes
          (Utilities|Casting|CastToReflectiveCube_BP _grabbedobjectvar)
          (Class|PhysicsHandleComponent|SetTargetRotation _physicshandle (Math|Rotator|MakeRotator 0.0 0.0 (.yaw (Math|Conversions|RotationFromXVector (* (- (Transformation|GetActorLocation (Game|GetPlayerCharacter 0)) (Transformation|GetActorLocation _grabbedobjectvar)) -1))))))))))

(fn SetupInputComponent)

(fn FindPhysicsHandleComponent
  (bind _output_get (Variables|Default|SetPhysicsHandle (Actor|GetComponentbyClass (Components|GetOwner) "/Script/Engine.PhysicsHandleComponent")))
  (Class|PhysicsHandleComponent|SetInterpolationSpeed _output_get 1e+02)
  (Utilities|IsValid _output_get
    (:Is%20Not%20Valid
      (Development|PrintString "ERROR! Could not find physics handle component on Grabber_BP!"))))

(fn DHandleGrab)

(fn Grab
  (params (ObjectToGrab :type Actor%20Object%20Reference))
  (bind _physicshandle (Variables|Default|GetPhysicsHandle))
  (Development|PrintString "Grabbing!")
  (bind _output_get (Variables|Default|SetGrabbedObjectVar ObjectToGrab))
  (Utilities|IsValid _output_get
    (:Is%20Valid
      (Utilities|IsValid _physicshandle
        (:Is%20Valid
          (Physics|Components|PhysicsHandle|GrabComponentatLocationwithRotation _physicshandle (Actor|GetComponentbyClass (Variables|Default|GetGrabbedObjectVar) "/Script/Engine.PrimitiveComponent") "None" (Transformation|GetActorLocation (Variables|Default|GetGrabbedObjectVar)) (Transformation|GetActorRotation (Variables|Default|GetGrabbedObjectVar)))
          (Variables|Default|SetMemoGrabbedComponent (Actor|GetComponentbyClass (Variables|Default|GetGrabbedObjectVar) "/Script/Engine.PrimitiveComponent"))
          (Variables|Default|SetMemoBoneName "None")
          (Variables|Default|SetMemoGrabbedLocation (Transformation|GetActorLocation (Variables|Default|GetGrabbedObjectVar)))
          (Variables|Default|SetMemoObjectRotation (Transformation|GetActorRotation (Variables|Default|GetGrabbedObjectVar))))
        (:Is%20Not%20Valid
          (Development|PrintString "ERROR! Physics Handle not set on Grabber_BP!"))))
    (:Is%20Not%20Valid
      (Development|PrintString "Hit Actor is INVALID!"))))

(fn Release
  (Physics|Components|PhysicsHandle|ReleaseComponent (Variables|Default|GetPhysicsHandle))
  (Variables|Default|SetGrabbedObjectVar 0))

(fn ReleaseTemporarily
  (Physics|Components|PhysicsHandle|ReleaseComponent (Variables|Default|GetPhysicsHandle)))

(fn GrabAfterTemporaryRelease
  (bind _physicshandle (Variables|Default|GetPhysicsHandle))
  (Physics|Components|PhysicsHandle|GrabComponentatLocationwithRotation _physicshandle (Variables|Default|GetMemoGrabbedComponent) (Variables|Default|GetMemoBoneName) (Variables|Default|GetMemoGrabbedLocation) (Variables|Default|GetMemoObjectRotation))
  (Development|PrintString (Utilities|String|ToString(Object) (Class|PhysicsHandleComponent|GetGrabbedComponent _physicshandle))))

(fn GetFirstPhysicsBodyinReach
  (bind _start (CallFunction|GetReachLineStart))
  (bind _end (CallFunction|GetReachLineEnd))
  (bind _outhit (Collision|LineTraceForObjects _start _end (Utilities|Array|MakeArray "ObjectTypeQuery4") false 0 "None"))
  (return _outhit))

(fn GetReachLineStart
  (bind _returnvalue (Actor|GetActorOfClass "/Game/FirstPersonCPP/Blueprints/FirstPersonCharacter.FirstPersonCharacter_C"))
  (return (Transformation|GetWorldLocation (Variables|/Script/Portals.PortalsCharacter|GetFirstPersonCameraComponent _returnvalue))))

(fn GetReachLineEnd
  (bind _returnvalue (Actor|GetActorOfClass "/Game/FirstPersonCPP/Blueprints/FirstPersonCharacter.FirstPersonCharacter_C"))
  (return (+ (* (Math|Vector|Normalize (Math|Vector|GetForwardVector (Variables|/Script/Portals.PortalsCharacter|GetFirstPersonCameraComponent _returnvalue))) (Variables|Default|GetReach)) (Transformation|GetWorldLocation (Variables|/Script/Portals.PortalsCharacter|GetFirstPersonCameraComponent _returnvalue)))))