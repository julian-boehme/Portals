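; Laser emitter that builds a chain of laser beam actors bouncing off reflector cubes, up to a fixed depth.
; UpdateLasers runs on BeginPlay, destroying old beams, re-tracing from the emitter's arrow, then enabling overlap listening on the new beams.
; MakeLineTrace spawns a beam per segment and recurses from each reflector hit, registering itself on that cube.
; Tick is empty, the facing-angle check is disconnected, and traces draw persistent debug lines.
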(event EventBeginPlay
  (CallFunction|UpdateLasers))

(event Collision|EventActorBeginOverlap
  (params (OtherActor :type Actor%20Object%20Reference)))

(event EventTick
  (params (DeltaSeconds :type Float%20%28single-precision%29)))

(fn ConstructionScript)

(fn MakeLineTrace
  (params (Start :type Vector) (Direction :type Vector) (CurrentTraceNr :type Integer) (MaxTraceDepth :type Integer) (IgnoredActor :type Actor%20Object%20Reference))
  (if (< CurrentTraceNr MaxTraceDepth)
    (bind _output_get (LocalVariables|SetEnd (+ Start (* Direction (Variables|Default|GetMaxTraceDistance)))))
    (bind (_outhit _returnvalue) (Collision|LineTraceByChannel Start _output_get "TraceTypeQuery3" false (Utilities|Array|MakeArray IgnoredActor) "Persistent"))
    (if _returnvalue
      (bind _returnvalue_2 (Game|SpawnActorfromClass "/Game/Portals/LaserEmitter/Laser_Ticking_BP.Laser_Ticking_BP_C" (Math|Transform|MakeTransform Start "0, 0, 0" "1,1,1") "Undefined" 0 Start (.Location (Collision|BreakHitResult _outhit)) self 0))
      (Utilities|Array|Add (Variables|Default|GetLaserBeams) 0)
      ;[1 1 1] Hit actor is ReflectorCube
      (bind _asreflector_cube_ticking_bp (Utilities|Casting|CastToReflectorCube_Ticking_BP (.HitActor (Collision|BreakHitResult _outhit))))
      (Variables|/Game/Portals/ReflectorCube_Ticking_BP.ReflectorCube_Ticking_BP_C|SetHittingLaserEmitter _asreflector_cube_ticking_bp self)
      (CallFunction|MakeLineTrace (Transformation|GetActorLocation _asreflector_cube_ticking_bp) (Math|Vector|GetForwardVector (Variables|Default|GetCube)) (+ CurrentTraceNr 1) MaxTraceDepth _asreflector_cube_ticking_bp)
      (else
        (Game|SpawnActorfromClass "/Game/Portals/LaserEmitter/Laser_Ticking_BP.Laser_Ticking_BP_C" (Math|Transform|MakeTransform Start "0, 0, 0" "1,1,1") "Undefined" 0 Start (LocalVariables|GetEnd) self 0)
        (Utilities|Array|Add (Variables|Default|GetLaserBeams) 0)
        (Default|CalculateLaser _returnvalue_2)))))

(fn DestroyLaserBeams
  (for _array_element (Variables|Default|GetLaserBeams)
    (Utilities|IsValid _array_element
      (:Is%20Valid
        (Rendering|SetActorHiddenInGame _array_element true)
        (Variables|/Game/Portals/LaserEmitter/Laser_BP.Laser_BP_C|SetListenForOverlap _array_element false)
        (Actor|DestroyActor _array_element)))))

(fn UpdateLasers
  (CallFunction|DestroyLaserBeams)
  (CallFunction|MakeLineTrace (Transformation|GetWorldLocation (Variables|Default|GetCube)) (Math|Vector|GetForwardVector (Variables|Default|GetArrow)) 0 5)
  (for _array_element (Variables|Default|GetLaserBeams)
    (Utilities|IsValid _array_element
      (:Is%20Valid
        (Variables|/Game/Portals/LaserEmitter/Laser_BP.Laser_BP_C|SetListenForOverlap _array_element true)))))