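; Moving platform actor that travels between StartPoint and EndPoint, optionally starting and stopping as the first-person player steps on or off.
; Timeline0, with play rate set from MovementSpeed, lerps the platform and reverses at each end.
; SetEnabled pauses or resumes it in the direction remembered in MemoDirection.
; The construction script places a hidden-in-game destination preview and orients and scales the rail along the path.
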(event OnComponentBeginOverlap(Box)
  (params (OverlappedComponent :type Primitive%20Component%20Object%20Reference) (OtherActor :type Actor%20Object%20Reference) (OtherComp :type Primitive%20Component%20Object%20Reference) (OtherBodyIndex :type Integer) (bFromSweep :type Boolean) (SweepResult :type Hit%20Result%20Structure%20%28by%20ref%29))
  ;[1 1 1] Player stepped on platform
  (if (Variables|Default|GetMoveWhenPlayerSteppedOn)
    (Utilities|Casting|CastToFirstPersonCharacter OtherActor)
    (Audio|Components|Audio|Play (Variables|Default|GetTimeline_0))))

(event OnComponentEndOverlap(Box)
  (params (OverlappedComponent :type Primitive%20Component%20Object%20Reference) (OtherActor :type Actor%20Object%20Reference) (OtherComp :type Primitive%20Component%20Object%20Reference) (OtherBodyIndex :type Integer))
  ;[1 1 1] Player left platform
  (if (Variables|Default|GetMoveWhenPlayerSteppedOn)
    (Utilities|Casting|CastToFirstPersonCharacter OtherActor)
    (Audio|Components|Audio|Stop (Variables|Default|GetTimeline_0))))

(event Custom|CustomEvent
  (params (OverlappedComponent :type Primitive%20Component%20Object%20Reference) (OtherActor :type Actor%20Object%20Reference) (OtherComp :type Primitive%20Component%20Object%20Reference) (OtherBodyIndex :type Integer) (bFromSweep :type Boolean) (SweepResult :type Hit%20Result%20Structure%20%28by%20ref%29))
  ;[1 1 1] DEPRECATED
  ;;[1 1 1] Player stepped on platform
  (Utilities|Casting|CastToFirstPersonCharacter OtherActor))

(event Custom|CustomEvent_1
  (params (OverlappedComponent :type Primitive%20Component%20Object%20Reference) (OtherActor :type Actor%20Object%20Reference) (OtherComp :type Primitive%20Component%20Object%20Reference) (OtherBodyIndex :type Integer))
  ;[1 1 1] DEPRECATED
  ;;[1 1 1] Player left platform
  (Utilities|Casting|CastToFirstPersonCharacter OtherActor))

(event EventBeginPlay
  ;[1 1 1] Position platform at StartPoint
  (Transformation|SetRelativeLocation (Variables|Default|GetPlatform) (Variables|Default|GetStartPoint) false false)
  ;[1 1 1] Apply movementSpeed by setting the PlayRate of the Timeline
  (Components|Timeline|SetPlayRate (Variables|Default|GetTimeline_0) (Variables|Default|GetMovementSpeed)))

(event Collision|EventActorBeginOverlap
  (params (OtherActor :type Actor%20Object%20Reference)))

(event EventTick
  (params (DeltaSeconds :type Float%20%28single-precision%29)))

(fn ConstructionScript
  (bind _rail (Variables|Default|GetRail))
  (bind _startpoint (Variables|Default|GetStartPoint))
  (bind _endpoint (Variables|Default|GetEndPoint))
  (bind _returnvalue (- _endpoint _startpoint))
  (bind _relativescale3d (Variables|/Script/Engine.SceneComponent|GetRelativeScale3D _rail))
  ;[1 1 1] Needs to be set here. Once I defined a constructor for this object, the "Hidden In Game" option in the "Details" panel doesn't work anymore.
  (Development|SetHiddeninGame (Variables|Default|GetDestinationPreview) true true)
  (Transformation|SetRelativeLocation (Variables|Default|GetDestinationPreview) (Variables|Default|GetEndPoint) false false)
  ;[1 1 1] Rotate Rails
  (Transformation|SetRelativeRotation (Variables|Default|GetRail) (Math|Rotator|MakeRotfromZ _returnvalue) false false)
  ;[1 1 1] Scale rails
  (Transformation|SetRelativeScale3D _rail (Math|Vector|MakeVector (.x _relativescale3d) (.y _relativescale3d) (/ (Math|Vector|VectorLength _returnvalue) (Variables|Default|GetDistanceToScaleConversionValue)))))

(fn SetEnabled
  (params (Enabled :type Boolean))
  (bind _timeline_0 (Variables|Default|GetTimeline_0))
  (bind _output_get (Variables|Default|SetEnabled Enabled))
  (if _output_get
    (if (Utilities|Enum|Equal(Enum) (Variables|Default|GetMemoDirection) "Forward")
      (Audio|Components|Audio|Play _timeline_0)
      (else
        (Utilities|String|Reverse _timeline_0)))
    (else
      (Audio|Components|Audio|Stop _timeline_0))))