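; EnergyBallSource_BP is an emitter actor that periodically fires EnergyBall_BP projectiles.
; On BeginPlay it starts a looping timer at the Interval; each tick, if Enabled, it spawns a ball at its Arrow component's transform.
; The spawn passes Lifespan, DestroyOnFirstHit and BallTarget to the ball, then sets its physics linear velocity along the arrow's forward vector scaled by Speed.
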(event Custom|OnTimerTick
  (bind _arrow (Variables|Default|GetArrow))
  (if (Variables|Default|GetEnabled)
    (bind _returnvalue (Game|SpawnActorfromClass "/Game/Portals/EnergyBall/EnergyBall_BP.EnergyBall_BP_C" (Transformation|GetWorldTransform _arrow) "Undefined" 0 (Variables|Default|GetLifespan) (Variables|Default|GetDestroyOnFirstHit) (Variables|Default|GetBallTarget) 0))
    (Physics|SetPhysicsLinearVelocity (Actor|GetComponentbyClass _returnvalue "/Script/Engine.PrimitiveComponent") (* (* (Math|Vector|GetForwardVector _arrow) (Variables|Default|GetSpeed)) 1) false "None")))

(event EventBeginPlay
  (Utilities|Time|SetTimerbyEvent (delegate Custom|OnTimerTick) (Math|Conversions|ToFloat(Integer) (Variables|Default|GetInterval)) true))

(event Collision|EventActorBeginOverlap
  (params (OtherActor :type Actor%20Object%20Reference)))

(event EventTick
  (params (DeltaSeconds :type Float%20%28single-precision%29)))

(fn ConstructionScript)