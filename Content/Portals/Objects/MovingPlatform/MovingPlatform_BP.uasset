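; Moving platform actor that travels back and forth between StartPoint and EndPoint along a rail, either oscillating or moving while the player stands on it.
; A timeline, with play rate set by MovementSpeed, lerps the platform and flips direction at each end, using MemoDirection to resume.
; SetOscillating toggles motion and light color from a material parameter collection.
; The construction script fits the rail to both points and places a hidden-in-game destination preview.
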(event OnComponentBeginOverlap(Box)
  (params (OverlappedComponent :type Primitive%20Component%20Object%20Reference) (OtherActor :type Actor%20Object%20Reference) (OtherComp :type Primitive%20Component%20Object%20Reference) (OtherBodyIndex :type Integer) (bFromSweep :type Boolean) (SweepResult :type Hit%20Result%20Structure%20%28by%20ref%29))
  ;[1 1 1] Player stepped on platform
  (if (Variables|Default|GetMoveWhenPlayerSteppedOn)
    (Utilities|Casting|CastToFirstPersonCharacter OtherActor)
    (Audio|Components|Audio|Play (Variables|Default|GetTimeline_0))))

(event OnComponentEndOverlap(Box)
  (params (OverlappedComponent :type Primitive%20Component%20Object%20Reference) (OtherActor :type Actor%20Object%20Reference) (OtherComp :type Primitive%20Component%20Object%20Reference) (OtherBodyIndex :type Integer))
  ;[1 1 1] Player left platform
  (if (Variables|Default|GetMoveWhenPlayerSteppedOn)
    (Utilities|Casting|CastToFirstPersonCharacter OtherActor)
    (Audio|Components|Audio|Stop (Variables|Default|GetTimeline_0))))

(event EventBeginPlay
  ;[1 1 1] Apply movementSpeed by setting the PlayRate of the Timeline
  (Components|Timeline|SetPlayRate (Variables|Default|GetTimeline_0) (Variables|Default|GetMovementSpeed))
  (if (Variables|Default|GetOscillating)
    (CallFunction|SetOscillating true)))

(event Collision|EventActorBeginOverlap
  (params (OtherActor :type Actor%20Object%20Reference)))

(event EventTick
  (params (DeltaSeconds :type Float%20%28single-precision%29)))

(fn ConstructionScript
  (bind _startpoint (Variables|Default|GetStartPoint))
  (bind _endpoint (Variables|Default|GetEndPoint))
  (bind _rail (Variables|Default|GetRail))
  (bind _returnvalue (- _endpoint _startpoint))
  (bind _relativescale3d (Variables|/Script/Engine.SceneComponent|GetRelativeScale3D _rail))
  (if (Variables|Default|GetOscillating)
    (CallFunction|SetLighttoActivatedColor)
    (else
      (CallFunction|SetLighttoDeactivatedColor)))
  ;[1 1 1] Needs to be set here. Once I defined a constructor for this object, the "Hidden In Game" option in the "Details" panel doesn't work anymore.
  (Development|SetHiddeninGame (Variables|Default|GetDestinationPreview) true true)
  ;[1 1 1] Position platform at StartPoint
  (Transformation|SetRelativeLocation (Variables|Default|GetPlatform) (Variables|Default|GetStartPoint) false false)
  ;[1 1 1] Position Preview
  (Transformation|SetRelativeLocation (Variables|Default|GetDestinationPreview) (Variables|Default|GetEndPoint) false false)
  ;[1 1 1] Rotate Rails
  (Transformation|SetRelativeRotation (Variables|Default|GetRail) (Math|Rotator|MakeRotfromZ _returnvalue) false false)
  ;[1 1 1] Scale rails
  (Transformation|SetRelativeScale3D _rail (Math|Vector|MakeVector (.x _relativescale3d) (.y _relativescale3d) (/ (Math|Vector|VectorLength _returnvalue) (Variables|Default|GetDistanceToScaleConversionValue))))
  ;[1 1 1] Set rail location
  (Transformation|SetRelativeLocation (Variables|Default|GetRail) (+ (Variables|Default|GetStartPoint) "0, 0,-50.000000") false true))

(fn SetOscillating
  (params (Oscillating :type Boolean))
  (bind _timeline_0 (Variables|Default|GetTimeline_0))
  (bind _output_get (Variables|Default|SetOscillating Oscillating))
  (if _output_get
    (CallFunction|SetLighttoActivatedColor)
    (if (Utilities|Enum|Equal(Enum) (Variables|Default|GetMemoDirection) "Forward")
      (Audio|Components|Audio|Play _timeline_0)
      (else
        (Utilities|String|Reverse _timeline_0)))
    (else
      (CallFunction|SetLighttoDeactivatedColor)
      (Audio|Components|Audio|Stop _timeline_0))))

(fn SetLighttoActivatedColor
  (bind _returnvalue (Rendering|Material|GetVectorParameterValue "/Game/Portals/MPC_Colors.MPC_Colors" "MovingPlatformActivatedColor" :!class /Script/Engine.KismetMaterialLibrary))
  (bind _returnvalue_2 (Rendering|Material|CreateDynamicMaterialInstance (Variables|Default|GetPlatform) (Variables|Default|GetPlatformLightMaterialIndex) "/Game/Portals/Models/MovingPlatform/MovingPlatformLight_mat.MovingPlatformLight_mat" "None" :!class /Script/Engine.PrimitiveComponent))
  (Rendering|Material|SetVectorParameterValue _returnvalue_2 "LightColor" _returnvalue :!class /Script/Engine.MaterialInstanceDynamic))

(fn SetLighttoDeactivatedColor
  (bind _returnvalue (Rendering|Material|GetVectorParameterValue "/Game/Portals/MPC_Colors.MPC_Colors" "MovingPlatformDeactivatedColor" :!class /Script/Engine.KismetMaterialLibrary))
  (bind _returnvalue_2 (Rendering|Material|CreateDynamicMaterialInstance (Variables|Default|GetPlatform) (Variables|Default|GetPlatformLightMaterialIndex) "/Game/Portals/Models/MovingPlatform/MovingPlatformLight_mat.MovingPlatformLight_mat" "None" :!class /Script/Engine.PrimitiveComponent))
  (Rendering|Material|SetVectorParameterValue _returnvalue_2 "LightColor" _returnvalue :!class /Script/Engine.MaterialInstanceDynamic))