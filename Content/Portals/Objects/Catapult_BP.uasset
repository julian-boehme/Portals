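; Catapult that flings the first-person player or physics objects that overlap its collision box, when enabled and ready.
; Players get LaunchCharacter with adjusted power; objects have velocity zeroed, then receive a mass-independent impulse for full force.
; Launch velocity pitches the local-space forward vector by Angle without converting back to world space; the construction script matches the arrow.
; A timeline swings the arm, waits for cooldown, then reverses before re-arming.
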(event OnComponentBeginOverlap(CollisionBox)
  (params (OverlappedComponent :type Primitive%20Component%20Object%20Reference) (OtherActor :type Actor%20Object%20Reference) (OtherComp :type Primitive%20Component%20Object%20Reference) (OtherBodyIndex :type Integer) (bFromSweep :type Boolean) (SweepResult :type Hit%20Result%20Structure%20%28by%20ref%29))
  (if (Variables|Default|GetEnabled)
    (Variables|Default|SetActor OtherActor)
    (if (Utilities|ClassIsChildOf (Utilities|GetClass OtherActor) "/Game/FirstPersonCPP/Blueprints/FirstPersonCharacter.FirstPersonCharacter_C")
      ;[1 1 1] Catapult Player
      (bind _asfirst_person_character (Utilities|Casting|CastToFirstPersonCharacter (Variables|Default|GetActor))
        (:then
          (if (Variables|Default|GetCanCatapult)
            (Variables|Default|SetCanCatapult false)
            (bind _velocityvector (CallFunction|CalculateLaunchVelocityVector (* (Variables|Default|GetJumpPower) (Variables|Default|GetPlayerJumpPowerAdjustment))))
            (Character|LaunchCharacter _asfirst_person_character _velocityvector true true)
            (bind (_direction _catapultangle) (Timeline|Timeline_0 PlayFromStart)
              (:Update
                (Transformation|SetRelativeRotation (Variables|Default|GetMovingPart) (Math|Rotator|MakeRotator 0.0 _catapultangle 0.0) false false))
              (:Finished
                (if (Utilities|Enum|Equal(Enum) _direction "Forward")
                  (Utilities|FlowControl|Delay (Variables|Default|GetCooldown))
                  (Timeline|Timeline_0 Reverse)
                  (else
                    (Variables|Default|SetCanCatapult true)))))))
        (:CastFailed
          (Development|PrintString "Cast failed")))
      (else
        ;[1 1 1] Catapult object
        (if (Variables|Default|GetCanCatapult)
          (Variables|Default|SetCanCatapult false)
          ;;[1 1 1] If an object falls onto the catapult, the object is not being catapulted with full force, but with the difference of the catapult power and its incoming velocity. To remedy this, set velocity to 0 before catapulting.
          (Physics|SetPhysicsLinearVelocity (Actor|GetComponentbyClass (Variables|Default|GetActor) "/Script/Engine.PrimitiveComponent") "0, 0, 0" false "None")
          (bind _velocityvector_2 (CallFunction|CalculateLaunchVelocityVector (Variables|Default|GetJumpPower)))
          (Physics|AddImpulse (Actor|GetComponentbyClass (Variables|Default|GetActor) "/Script/Engine.PrimitiveComponent") _velocityvector_2 "None" true)
          (Timeline|Timeline_0 PlayFromStart))))))

(event EventBeginPlay)

(event Collision|EventActorBeginOverlap
  (params (OtherActor :type Actor%20Object%20Reference)))

(event EventTick
  (params (DeltaSeconds :type Float%20%28single-precision%29)))

(fn ConstructionScript
  ;[1 1 1] Set Arrow rotation to Angle Parameter
  (Transformation|SetRelativeRotation (Variables|Default|GetArrow) (Math|Rotator|MakeRotator 0.0 (Variables|Default|GetAngle) 0.0) false false))

(fn CalculateLaunchVelocityVector
  (params (JumpPower :type Float%20%28single-precision%29))
  (return (* (Math|Vector|RotateVector (Math|Transform|InverseTransformDirection (Transformation|GetActorTransform) (Transformation|GetActorForwardVector)) (Math|Rotator|MakeRotator 0.0 (Variables|Default|GetAngle) 0.0)) (* JumpPower (LocalVariables|GetJumpPowerIncreaser)))))