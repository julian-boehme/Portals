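; Sliding double door that opens for the first-person character when unlocked and closes itself after a short delay.
; A box overlap starts chained timelines that lerp the lock piece open, then both door halves, and later reverse in the opposite order through separate close timelines.
; SetLocked, also run by the Construction Script, stores the lock state and switches red and green indicator lights through dynamic material instances.
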(event OnComponentBeginOverlap(Box)
  (params (OverlappedComponent :type Primitive%20Component%20Object%20Reference) (OtherActor :type Actor%20Object%20Reference) (OtherComp :type Primitive%20Component%20Object%20Reference) (OtherBodyIndex :type Integer) (bFromSweep :type Boolean) (SweepResult :type Hit%20Result%20Structure%20%28by%20ref%29))
  (if (not (Variables|Default|GetLocked))
    (Utilities|Casting|CastToFirstPersonCharacter OtherActor)
    ;[1 1 1] Open lock
    (bind _lockdisplacement (Timeline|LockOpenTimeline PlayFromStart)
      (:Update
        (Transformation|SetRelativeLocation (Variables|Default|Getlock_moving_part) (Math|Vector|Lerp(Vector) (Variables|Default|GetLockClosedPos) (Variables|Default|GetLockOpenPos) _lockdisplacement) false false))
      (:Finished
        (Utilities|FlowControl|Sequence
          (:then_0
            ;[1 1 1] Open left door
            (bind _doordisplacement (Timeline|LeftDoorOpenTimeline PlayFromStart)
              (:Update
                (Transformation|SetRelativeLocation (Variables|Default|Getdoor_left) (Math|Vector|Lerp(Vector) (Variables|Default|GetDoorLeftClosedPos) (Variables|Default|GetDoorLeftOpenPos) _doordisplacement) false false))))
          (:then_1
            ;[1 1 1] Open right door
            (bind _doordisplacement_2 (Timeline|RightDoorTimeline PlayFromStart)
              (:Update
                (Transformation|SetRelativeLocation (Variables|Default|Getdoor_right) (Math|Vector|Lerp(Vector) (Variables|Default|GetDoorRightClosedPos) (Variables|Default|GetDoorRightOpenPos) _doordisplacement_2) false false))
              (:Finished
                (Utilities|FlowControl|Delay 2.0)
                (Utilities|FlowControl|Sequence
                  (:then_0
                    ;[1 1 1] Close left door
                    (bind _doordisplacement_3 (Timeline|DoorLeftCloseTimeline ReverseFromEnd)
                      (:Update
                        (Transformation|SetRelativeLocation (Variables|Default|Getdoor_left) (Math|Vector|Lerp(Vector) (Variables|Default|GetDoorLeftClosedPos) (Variables|Default|GetDoorLeftOpenPos) _doordisplacement_3) false false))))
                  (:then_1
                    ;[1 1 1] Close right door
                    (bind _doordisplacement_4 (Timeline|DoorRightCloseTimeline ReverseFromEnd)
                      (:Update
                        (Transformation|SetRelativeLocation (Variables|Default|Getdoor_right) (Math|Vector|Lerp(Vector) (Variables|Default|GetDoorRightClosedPos) (Variables|Default|GetDoorRightOpenPos) _doordisplacement_4) false false))
                      (:Finished
                        ;[1 1 1] Close lock
                        (bind _lockdisplacement_2 (Timeline|LockCloseTimeline ReverseFromEnd)
                          (:Update
                            (Transformation|SetRelativeLocation (Variables|Default|Getlock_moving_part) (Math|Vector|Lerp(Vector) (Variables|Default|GetLockClosedPos) (Variables|Default|GetLockOpenPos) _lockdisplacement_2) false false)))))))))))))))

(event EventBeginPlay)

(event Collision|EventActorBeginOverlap
  (params (OtherActor :type Actor%20Object%20Reference)))

(event EventTick
  (params (DeltaSeconds :type Float%20%28single-precision%29)))

(fn ConstructionScript
  (CallFunction|SetLocked (Variables|Default|GetLocked)))

(fn SetLocked
  (params (Locked :type Boolean))
  (bind _door_top (Variables|Default|Getdoor_top))
  (bind _door_top_2 (Variables|Default|Getdoor_top))
  (bind _output_get (Variables|Default|SetLocked Locked))
  (if _output_get
    ;[1 1 1] Update lights: Lock
    (Utilities|FlowControl|Sequence
      (:then_0
        (bind _returnvalue (Rendering|Material|CreateDynamicMaterialInstance _door_top (Variables|Default|GetRedLightMaterialIndex) "/Game/Portals/Models/Door/Door_RedLight_mat.Door_RedLight_mat" "None" :!class /Script/Engine.PrimitiveComponent))
        (Rendering|Material|SetScalarParameterValue _returnvalue "LightStrength" (LocalVariables|GetLightStrength) :!class /Script/Engine.MaterialInstanceDynamic))
      (:then_1
        (bind _returnvalue_2 (Rendering|Material|CreateDynamicMaterialInstance _door_top (Variables|Default|GetGreenLightMaterialIndex) "/Game/Portals/Models/Door/Door_GreenLight_mat.Door_GreenLight_mat" "None" :!class /Script/Engine.PrimitiveComponent))
        (Rendering|Material|SetScalarParameterValue _returnvalue_2 "LightStrength" 0.0 :!class /Script/Engine.MaterialInstanceDynamic)))
    (else
      ;[1 1 1] Update lights: Unlock
      (Utilities|FlowControl|Sequence
        (:then_0
          (bind _returnvalue_3 (Rendering|Material|CreateDynamicMaterialInstance _door_top_2 (Variables|Default|GetRedLightMaterialIndex) "/Game/Portals/Models/Door/Door_RedLight_mat.Door_RedLight_mat" "None" :!class /Script/Engine.PrimitiveComponent))
          (Rendering|Material|SetScalarParameterValue _returnvalue_3 "LightStrength" 0.0 :!class /Script/Engine.MaterialInstanceDynamic))
        (:then_1
          (bind _returnvalue_4 (Rendering|Material|CreateDynamicMaterialInstance _door_top_2 (Variables|Default|GetGreenLightMaterialIndex) "/Game/Portals/Models/Door/Door_GreenLight_mat.Door_GreenLight_mat" "None" :!class /Script/Engine.PrimitiveComponent))
          (Rendering|Material|SetScalarParameterValue _returnvalue_4 "LightStrength" (LocalVariables|GetLightStrength) :!class /Script/Engine.MaterialInstanceDynamic))))))