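; Modular wall builder for a portal game that lays out a grid of black panels with optional holes and white portal-spawnable tiles.
; The construction script loops over rows and columns, skipping cells in Holes and adding white wall instances for cells in PortalSpawnableSurfaces, black otherwise.
; Black cells on the grid's outer edges also get optional top, bottom, left and right beam instances through helper functions.
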(event EventBeginPlay)

(event Collision|EventActorBeginOverlap
  (params (OtherActor :type Actor%20Object%20Reference)))

(event EventTick
  (params (DeltaSeconds :type Float%20%28single-precision%29)))

(fn ConstructionScript
  ;[1 1 1] Height
  (for _index (range 0 (- (Variables|Default|GetNumAlongZ) 1))
    (LocalVariables|SetCurrentRow _index)
    (LocalVariables|SetCurrentRowOffset (* (Variables|Default|GetObjectOffsetZ) _index))
    ;[1 1 1] Width
    (for _index_2 (range 0 (- (Variables|Default|GetNumAlongY) 1))
      (bind _output_get (LocalVariables|SetCurrentColumn _index_2))
      (bind _ishole (CallFunction|IsHole _output_get (LocalVariables|GetCurrentRow)))
      (if (not _ishole)
        (LocalVariables|SetSpawnLocation (+ (* (Variables|Default|GetObjectOffsetY) (LocalVariables|GetCurrentColumn)) (LocalVariables|GetCurrentRowOffset)))
        (bind _isnonportalspawnablesurface (CallFunction|IsPortalSpawnableSurface (LocalVariables|GetCurrentColumn) (LocalVariables|GetCurrentRow)))
        (if _isnonportalspawnablesurface
          (Components|InstancedStaticMesh|AddInstance (Variables|Default|GetWhiteWall) (Math|Transform|MakeTransform (LocalVariables|GetSpawnLocation) "0, 0, 0" "1,1,1"))
          (else
            (Components|InstancedStaticMesh|AddInstance (Variables|Default|GetBlackWall) (Math|Transform|MakeTransform (LocalVariables|GetSpawnLocation) "0, 0, 0" "1,1,1"))
            (CallFunction|CreateBeamTop (LocalVariables|GetCurrentRow) (LocalVariables|GetSpawnLocation))
            (CallFunction|CreateBeamBottom (LocalVariables|GetCurrentRow) (LocalVariables|GetSpawnLocation))
            (CallFunction|CreateBeamLeft (LocalVariables|GetCurrentColumn) (LocalVariables|GetSpawnLocation))
            (CallFunction|CreateBeamRight (LocalVariables|GetCurrentColumn) (LocalVariables|GetSpawnLocation))))))))

(fn IsHole
  (params (Column :type Integer) (Row :type Integer))
  (for _array_element (Variables|Default|GetHoles)
    (if (and (== (.X (Math|Vector|BreakVector _array_element)) (Math|Conversions|ToFloat(Integer) Column)) (== (.Y (Math|Vector|BreakVector _array_element)) (Math|Conversions|ToFloat(Integer) Row)))
      (return true)))
  (return false))

(fn IsPortalSpawnableSurface
  (params (Column :type Integer) (Row :type Integer))
  (for _array_element (Variables|Default|GetPortalSpawnableSurfaces)
    (if (and (== (.X (Math|Vector|BreakVector _array_element)) (Math|Conversions|ToFloat(Integer) Column)) (== (.Y (Math|Vector|BreakVector _array_element)) (Math|Conversions|ToFloat(Integer) Row)))
      (return true)))
  (return false))

(fn CreateBeamTop
  (params (CurrentRow :type Integer) (SpawnLocation :type Vector))
  (if (and (== CurrentRow (- (Variables|Default|GetNumAlongZ) 1)) (Variables|Default|GetAddBeamTop))
    (Components|InstancedStaticMesh|AddInstance (Variables|Default|GetBeamTop) (Math|Transform|MakeTransform SpawnLocation "0, 0, 0" "1,1,1")))
  (return))

(fn CreateBeamBottom
  (params (CurrentRow :type Integer) (SpawnLocation :type Vector))
  (if (and (== CurrentRow 0) (Variables|Default|GetAddBeamBottom))
    (Components|InstancedStaticMesh|AddInstance (Variables|Default|GetBeamBottom) (Math|Transform|MakeTransform SpawnLocation "0, 0, 0" "1,1,1")))
  (return))

(fn CreateBeamRight
  (params (CurrentColumn :type Integer) (SpawnLocation :type Vector))
  (if (and (== CurrentColumn 0) (Variables|Default|GetAddBeamRight))
    (Components|InstancedStaticMesh|AddInstance (Variables|Default|GetBeamRight) (Math|Transform|MakeTransform (+ SpawnLocation (Variables|Default|GetRightBeamOffsetLocation)) "0, 0, 0" "1,1,1")))
  (return))

(fn CreateBeamLeft
  (params (CurrentColumn :type Integer) (SpawnLocation :type Vector))
  (if (and (== CurrentColumn (- (Variables|Default|GetNumAlongY) 1)) (Variables|Default|GetAddBeamLeft))
    (Components|InstancedStaticMesh|AddInstance (Variables|Default|GetBeamLeft) (Math|Transform|MakeTransform (+ SpawnLocation (Variables|Default|GetLeftBeamOffsetLocation)) "0, 0, 0" "1,1,1")))
  (return))