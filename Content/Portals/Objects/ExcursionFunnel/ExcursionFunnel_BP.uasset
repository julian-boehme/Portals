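; Portal-style excursion funnel emitter that projects a tube actor from its outer ring and spins its inner rings while enabled.
; Starting spawns TubeA, which a line trace centers and scales to the first hit or maximum length.
; Reverse flips ring rotation and updates tube color.
; Portal visibility events remove TubeB; its spawning and the portal-spawning handler are empty stubs.
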(event Custom|OnPortalVisibilityChangedB
  (bind _tubeb (Variables|Default|GetTubeB))
  ;[1 1 1] Bind Event Portal OnSetVisible
  ;[1 1 1] Remove TubeB if Portal location is changing or if Portal has been destroyed
  (Utilities|IsValid _tubeb
    (:Is%20Valid
      (Development|PrintString "Removing Tube B" true true "(R=0.170000,G=0.100721,B=1.000000,A=1.000000)")
      (Variables|/Game/Portals/Objects/ExcursionFunnel/ExcursionFunnelTube_BP.ExcursionFunnelTube_BP_C|SetEnabled _tubeb false)
      (Collision|SetCollisionEnabled (Variables|/Game/Portals/Objects/ExcursionFunnel/ExcursionFunnelTube_BP.ExcursionFunnelTube_BP_C|GetCylinder _tubeb) "NoCollision")
      (Rendering|SetVisibility (Variables|/Script/Engine.Actor|GetRootComponent _tubeb) false true)
      (Actor|DestroyActor (Variables|Default|GetTubeB)))))

(event Custom|OnPortalSpawning)

(event Custom|OnPortalVisibilityChangedA
  (bind _tubeb (Variables|Default|GetTubeB))
  ;[1 1 1] Bind Event Portal OnSetVisible
  ;[1 1 1] Remove TubeB if Portal location is changing or if Portal has been destroyed
  (Utilities|IsValid _tubeb
    (:Is%20Valid
      (Development|PrintString "Removing Tube B" true true "(R=0.170000,G=0.100721,B=1.000000,A=1.000000)")
      (Variables|/Game/Portals/Objects/ExcursionFunnel/ExcursionFunnelTube_BP.ExcursionFunnelTube_BP_C|SetEnabled _tubeb false)
      (Collision|SetCollisionEnabled (Variables|/Game/Portals/Objects/ExcursionFunnel/ExcursionFunnelTube_BP.ExcursionFunnelTube_BP_C|GetCylinder _tubeb) "NoCollision")
      (Rendering|SetVisibility (Variables|/Script/Engine.Actor|GetRootComponent _tubeb) false true)
      (Actor|DestroyActor (Variables|Default|GetTubeB)))))

(event EventBeginPlay
  ;[1 1 1] Start Funnel
  (if (Variables|Default|GetEnabled)
    (CallFunction|StartExcursionFunnel)
    (Utilities|FlowControl|Sequence
      (:then_0
        (bind _returnvalue (Actor|GetActorOfClass "/Game/Portals/Objects/Portals/Portal_A_BP_Child.Portal_A_BP_Child_C"))
        (Utilities|IsValid _returnvalue
          (:Is%20Valid
            (bind _output_get (Variables|Default|SetPortalA _returnvalue))
            ;[1 1 1] Bind Event Portal OnSetVisible
            (EventDispatchers|BindEventtoOnSetVisible _output_get (delegate Custom|OnPortalVisibilityChangedA)))
          (:Is%20Not%20Valid
            (Development|PrintString "ERROR! [Excursion Funnel - BeingPlay] Could not find Portal A in level." true true "(R=1.000000,G=0.000000,B=0.059606,A=1.000000)"))))
      (:then_1
        (bind _returnvalue_2 (Actor|GetActorOfClass "/Game/Portals/Objects/Portals/Portal_B_BP_Child.Portal_B_BP_Child_C"))
        (Utilities|IsValid _returnvalue_2
          (:Is%20Valid
            (bind _output_get_2 (Variables|Default|SetPortalB _returnvalue_2))
            ;[1 1 1] Bind Event Portal OnSetVisible
            (EventDispatchers|BindEventtoOnSetVisible _output_get_2 (delegate Custom|OnPortalVisibilityChangedB)))))
      (:then_2
        ;[1 1 1] Bind Event Portal OnPortalSpawning
        (bind _asfirst_person_character (Utilities|Casting|CastToFirstPersonCharacter (Game|GetPlayerCharacter 0)))
        (EventDispatchers|BindEventtoPortalSpawning _asfirst_person_character (delegate Custom|OnPortalSpawning))))))

(event Collision|EventActorBeginOverlap
  (params (OtherActor :type Actor%20Object%20Reference)))

(event EventTick
  (params (DeltaSeconds :type Float%20%28single-precision%29)))

(fn ConstructionScript)

(fn DReleasePlayer
  (params (Player :type First%20Person%20Character%20Object%20Reference))
  (bind _capsulecomponent (Variables|/Script/Engine.Character|GetCapsuleComponent Player))
  (Physics|SetSimulatePhysics _capsulecomponent false)
  (Physics|SetEnableGravity _capsulecomponent true))

(fn SetTubeTransform
  (params (Tube :type Excursion%20Funnel%20Tube%20BP%20Object%20Reference) (StartLocation :type Vector) (TraceDirection :type Vector))
  (LocalVariables|SetTubeVar Tube)
  (LocalVariables|SetStartLocationVar StartLocation)
  (LocalVariables|SetTraceDirectionVar TraceDirection)
  ;[1 1 1] Find first static object / wall the tube hits.
  (bind (_outhit _returnvalue) (Collision|LineTraceForObjects (LocalVariables|GetStartLocationVar) (+ (LocalVariables|GetStartLocationVar) (* (LocalVariables|GetTraceDirectionVar) (LocalVariables|GetLineTraceLength))) (Utilities|Array|MakeArray "ObjectTypeQuery1" "ObjectTypeQuery2") false 0 "None"))
  (if _returnvalue
    ;[1 1 1] Line trace hit wall. Calculate bridge length and position.
    (LocalVariables|SetScalingFactorZ (/ (.Distance (Collision|BreakHitResult _outhit)) (LocalVariables|GetDistanceToScaleConversionValue)))
    (Transformation|SetActorLocationAndRotation (LocalVariables|GetTubeVar) (+ (LocalVariables|GetStartLocationVar) (/ (- (.Location (Collision|BreakHitResult _outhit)) (LocalVariables|GetStartLocationVar)) 2)) (Math|Rotator|MakeRotator (.roll (Transformation|GetActorRotation)) (.pitch (Math|Conversions|RotationFromXVector (LocalVariables|GetTraceDirectionVar))) (.yaw (Math|Conversions|RotationFromXVector (LocalVariables|GetTraceDirectionVar)))))
    (Transformation|SetActorRelativeScale3D (LocalVariables|GetTubeVar) (Math|Vector|MakeVector (LocalVariables|GetScalingFactorZ) 1.0 1.0))
    (else
      ;[1 1 1] Line trace didn't hit anything. Extend tube to maximum length.
      (LocalVariables|SetScalingFactorZ (/ (Variables|Default|GetMaxTubeLength) (LocalVariables|GetDistanceToScaleConversionValue)))
      (Transformation|SetActorLocationAndRotation (LocalVariables|GetTubeVar) (+ (LocalVariables|GetStartLocationVar) (* TraceDirection (/ (Variables|Default|GetMaxTubeLength) 2.0))) (Math|Rotator|MakeRotator (.roll (Transformation|GetActorRotation)) (.pitch (Math|Conversions|RotationFromXVector (LocalVariables|GetTraceDirectionVar))) (.yaw (Math|Conversions|RotationFromXVector (LocalVariables|GetTraceDirectionVar)))))
      (Transformation|SetActorRelativeScale3D (LocalVariables|GetTubeVar) (Math|Vector|MakeVector (LocalVariables|GetScalingFactorZ) 1.0 1.0)))))

(fn SpawnTubeA
  (bind _returnvalue (Game|SpawnActorfromClass "/Game/Portals/Objects/ExcursionFunnel/ExcursionFunnelTube_BP.ExcursionFunnelTube_BP_C" (Math|Transform|MakeTransform "0, 0, 0" (Transformation|GetActorRotation) "1,1,1") "Undefined" 0 self (Math|Vector|GetForwardVector (Variables|Default|GetArrow)) 0))
  (bind _output_get (Variables|Default|SetTubeA _returnvalue))
  (CallFunction|SetTubeTransform _output_get (Transformation|GetWorldLocation (Variables|Default|GetOuterRing)) (Math|Vector|GetForwardVector (Variables|Default|GetArrow))))

(fn SpawnTubeB)

(fn SetEnabled
  (params (Enabled :type Boolean))
  (Variables|Default|SetEnabled Enabled)
  (if Enabled
    _))

(fn IsEnabled
  (return (Variables|Default|GetEnabled)))

(fn StartExcursionFunnel
  (Variables|Default|SetEnabled true)
  ;[1 1 1] Animation
  (Components|Movement|SetUpdatedComponent (Variables|Default|GetRotatingComponentInnerRing) (Variables|Default|GetInnerRing))
  (Components|Movement|SetUpdatedComponent (Variables|Default|GetRotatingComponentMiddleRing) (Variables|Default|GetMiddleRing))
  (CallFunction|UpdateMechanicsRotation)
  ;[1 1 1] Spawn Tube A
  (Utilities|IsValid (Variables|Default|GetTubeA)
    (:Is%20Not%20Valid
      (CallFunction|SpawnTubeA)
      (CallFunction|SetForceDirection (Variables|Default|GetReverse)))))

(fn StopExcursionFunnel
  (bind _tubea (Variables|Default|GetTubeA))
  (bind _tubeb (Variables|Default|GetTubeB))
  (Variables|Default|SetEnabled false)
  (Utilities|FlowControl|Sequence
    (:then_0
      (Utilities|IsValid _tubea
        (:Is%20Valid
          (Actor|DestroyActor _tubea))))
    (:then_1
      (Utilities|IsValid _tubeb
        (:Is%20Valid
          (Actor|DestroyActor _tubeb))))
    (:then_2
      (Variables|/Script/Engine.RotatingMovementComponent|SetRotationRate (Variables|Default|GetRotatingComponentInnerRing) "0, 0, 0")
      (Variables|/Script/Engine.RotatingMovementComponent|SetRotationRate (Variables|Default|GetRotatingComponentMiddleRing) "0, 0, 0"))))

(fn UpdateMechanicsRotation
  (if (Variables|Default|GetReverse)
    (Variables|/Script/Engine.RotatingMovementComponent|SetRotationRate (Variables|Default|GetRotatingComponentInnerRing) (* (Variables|Default|GetRotationRateInnerRing) -1))
    (Variables|/Script/Engine.RotatingMovementComponent|SetRotationRate (Variables|Default|GetRotatingComponentMiddleRing) (* (Variables|Default|GetRotationRateMiddleRing) -1))
    (else
      (Variables|/Script/Engine.RotatingMovementComponent|SetRotationRate (Variables|Default|GetRotatingComponentInnerRing) (Variables|Default|GetRotationRateInnerRing))
      (Variables|/Script/Engine.RotatingMovementComponent|SetRotationRate (Variables|Default|GetRotatingComponentMiddleRing) (Variables|Default|GetRotationRateMiddleRing)))))

(fn SetForceDirection
  (params (Reverse :type Boolean))
  (bind _tubeb (Variables|Default|GetTubeB))
  (bind _tubea (Variables|Default|GetTubeA))
  (Variables|Default|SetReverse Reverse)
  (if (Variables|Default|GetEnabled)
    (CallFunction|UpdateMechanicsRotation))
  (Utilities|IsValid _tubea
    (:Is%20Valid
      (Default|UpdateTubeColor _tubea Reverse)
      (Utilities|IsValid _tubeb
        (:Is%20Valid
          (Default|UpdateTubeColor _tubeb Reverse))))))