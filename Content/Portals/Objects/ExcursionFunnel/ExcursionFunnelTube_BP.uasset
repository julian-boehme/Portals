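; Tube volume of a Portal-style excursion funnel that carries the player and physics objects along its length.
; While enabled, Tick pushes overlapping actors, skipping portals and held objects, by disabling gravity, zeroing velocity and applying the parent funnel's forward or reverse force.
; Objects are re-centered every tick, the player only on entry; moving or exiting releases the player until re-entry.
; BeginPlay colors the tube by direction from a material parameter collection.
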(event OnComponentBeginOverlap(Cylinder)
  (params (OverlappedComponent :type Primitive%20Component%20Object%20Reference) (OtherActor :type Actor%20Object%20Reference) (OtherComp :type Primitive%20Component%20Object%20Reference) (OtherBodyIndex :type Integer) (bFromSweep :type Boolean) (SweepResult :type Hit%20Result%20Structure%20%28by%20ref%29))
  ;[1 1 1] Make sure player can re-enter tube after leaving.
  (Utilities|Casting|CastToFirstPersonCharacter OtherActor)
  (Variables|Default|SetDropPlayer false)
  (CallFunction|MoveActortoCenterOfTube OtherActor))

(event OnComponentEndOverlap(Cylinder)
  (params (OverlappedComponent :type Primitive%20Component%20Object%20Reference) (OtherActor :type Actor%20Object%20Reference) (OtherComp :type Primitive%20Component%20Object%20Reference) (OtherBodyIndex :type Integer))
  (bind _output_get (Variables|Default|SetActor OtherActor))
  (bind _asfirst_person_character (Utilities|Casting|CastToFirstPersonCharacter _output_get)
    (:then
      ;[1 1 1] Drop player
      (CallFunction|ReleasePlayer _asfirst_person_character))
    (:CastFailed
      ;[1 1 1] Drop objects
      (Physics|SetSimulatePhysics (Actor|GetComponentbyClass (Variables|Default|GetActor) "/Script/Engine.PrimitiveComponent") true)
      (Physics|SetEnableGravity (Actor|GetComponentbyClass (Variables|Default|GetActor) "/Script/Engine.PrimitiveComponent") true))))

(event Custom|OnPlayerMovement
  ;[1 1 1] Release Player when he tries to move.
  ;;[1 1 1] Is player currently in Anti-Gravitiy-Tube?
  (if (Utilities|Array|ContainsItem (Collision|GetOverlappingActors 0 :!class /Script/Engine.Actor) (stale EventBeginPlay _asfirst_person_character))
    (CallFunction|ReleasePlayer (stale EventBeginPlay _asfirst_person_character))))

(event EventBeginPlay
  (CallFunction|UpdateTubeColor (Variables|/Game/Portals/Objects/ExcursionFunnel/ExcursionFunnel_BP.ExcursionFunnel_BP_C|GetReverse (Variables|Default|GetParentFunnel)))
  ;[1 1 1] Release Player when he tries to move.
  (bind _asfirst_person_character (Utilities|Casting|CastToFirstPersonCharacter (Game|GetPlayerCharacter 0)))
  (EventDispatchers|BindEventtoPlayerMoving _asfirst_person_character (delegate Custom|OnPlayerMovement)))

(event Collision|EventActorBeginOverlap
  (params (OtherActor :type Actor%20Object%20Reference)))

(event EventTick
  (params (DeltaSeconds :type Float%20%28single-precision%29))
  (bind _enabled (Default|IsEnabled (Variables|Default|GetParentFunnel)))
  (if (and _enabled (Variables|Default|GetEnabled))
    (for _array_element (Collision|GetOverlappingActors 0 :!class /Script/Engine.Actor)
      ;[1 1 1] Make sure object is not held by player
      (bind _asfirst_person_character (Utilities|Casting|CastToFirstPersonCharacter (Game|GetPlayerCharacter 0)))
      (if (!= _array_element (Variables|/Game/Portals/Objects/Grabber_BP.Grabber_BP_C|GetGrabbedObject (Variables|/Game/FirstPersonCPP/Blueprints/FirstPersonCharacter.FirstPersonCharacter_C|GetGrabber_BP _asfirst_person_character)))
        (bind _output_get (Variables|Default|SetActor _array_element))
        (Utilities|Casting|CastToPortalSuperclass _output_get ; Ignore Portals, otherwise the funnel might try to push e.g. the Portal's arrow.
          (:CastFailed
            (bind _asfirst_person_character_2 (Utilities|Casting|CastToFirstPersonCharacter _output_get)
              (:then
                (if (not (Variables|Default|GetDropPlayer))
                  ;[1 1 1] Actor is FirstPersonCharacter
                  (bind _output_get_2 (Variables|Default|SetPlayerInTube _asfirst_person_character_2))
                  (CallFunction|PushPlayer _output_get_2)))
              (:CastFailed
                ;[1 1 1] Actor is object
                (CallFunction|PushObject (Variables|Default|GetActor))))))))))

(fn ConstructionScript
  (Variables|Default|SetReverseForceDirection (* (Variables|Default|GetOriginalForceDirection) -1)))

(fn MoveActortoCenterOfTube
  (params (Actor :type Actor%20Object%20Reference))
  (bind _defaultsceneroot (Variables|Default|GetDefaultSceneRoot))
  (bind _returnvalue (Transformation|GetWorldTransform _defaultsceneroot))
  (Transformation|SetActorLocation Actor (Math|Transform|TransformLocation _returnvalue (Math|Vector|MakeVector (.x (Math|Transform|InverseTransformLocation _returnvalue (Transformation|GetActorLocation Actor))) 0.0 0.0)) false true))

(fn CalculateForceStrength
  (bind _parentfunnel (Variables|Default|GetParentFunnel))
  (if (Variables|/Game/Portals/Objects/ExcursionFunnel/ExcursionFunnel_BP.ExcursionFunnel_BP_C|GetReverse (Variables|Default|GetParentFunnel))
    (LocalVariables|SetDirection (Variables|Default|GetReverseForceDirection))
    (else
      (LocalVariables|SetDirection (Variables|Default|GetOriginalForceDirection))))
  (return (* (LocalVariables|GetDirection) (* (Variables|/Game/Portals/Objects/ExcursionFunnel/ExcursionFunnel_BP.ExcursionFunnel_BP_C|GetForceStrength _parentfunnel) (Variables|/Game/Portals/Objects/ExcursionFunnel/ExcursionFunnel_BP.ExcursionFunnel_BP_C|GetForceIncreaser _parentfunnel)))))

(fn ReleasePlayer
  (params (Player :type First%20Person%20Character%20Object%20Reference))
  (bind _capsulecomponent (Variables|/Script/Engine.Character|GetCapsuleComponent Player))
  (Physics|SetSimulatePhysics _capsulecomponent false)
  (Physics|SetEnableGravity _capsulecomponent true)
  (Variables|Default|SetDropPlayer true))

(fn ReleaseObject
  (params (Actor :type Actor%20Object%20Reference))
  (bind _returnvalue (Actor|GetComponentbyClass Actor "/Script/Engine.PrimitiveComponent"))
  (Physics|SetSimulatePhysics _returnvalue true)
  (Physics|SetEnableGravity _returnvalue true)
  (Physics|SetPhysicsLinearVelocity _returnvalue "0, 0, 0" false "None"))

(fn PushPlayer
  (params (Character :type Character%20Object%20Reference))
  (bind _capsulecomponent (Variables|/Script/Engine.Character|GetCapsuleComponent Character))
  (Physics|SetSimulatePhysics _capsulecomponent true)
  (Physics|SetEnableGravity _capsulecomponent false)
  ;[1 1 1] Set velocity to 0 before adding Force to avoid increasing it with every tick.
  (Variables|/Script/Engine.MovementComponent|SetVelocity (Pawn|GetMovementComponent Character) "0, 0, 0")
  (Physics|SetPhysicsLinearVelocity _capsulecomponent "0, 0, 0" false "None") ; Remove any velocity the player had.
  (bind _force (CallFunction|CalculateForceStrength))
  (Physics|AddForce _capsulecomponent _force "None" true))

(fn PushObject
  (params (Actor :type Actor%20Object%20Reference))
  (bind _returnvalue (Actor|GetComponentbyClass Actor "/Script/Engine.PrimitiveComponent"))
  (bind _returnvalue_2 (Collision|GetCollisionEnabled _returnvalue))
  (if (and (or (Utilities|Enum|Equal(Enum) _returnvalue_2 "PhysicsOnly") (Utilities|Enum|Equal(Enum) _returnvalue_2 "QueryAndPhysics")) (Utilities|Enum|NotEqual(Enum) (Collision|GetCollisionObjectType _returnvalue) "ECC_WorldStatic"))
    (Physics|SetSimulatePhysics _returnvalue true)
    (Physics|SetEnableGravity _returnvalue false)
    (CallFunction|MoveActortoCenterOfTube (Variables|Default|GetActor))
    ;[1 1 1] Set velocity to 0 before adding Force to avoid increasing it with every tick.
    (Physics|SetPhysicsLinearVelocity _returnvalue "0, 0, 0" false "None")
    (bind _force (CallFunction|CalculateForceStrength))
    (Physics|AddForce _returnvalue _force "None" true)))

(fn UpdateTubeColor
  (params (Reverse :type Boolean))
  (bind _returnvalue (Rendering|Material|CreateDynamicMaterialInstance (Variables|Default|GetCylinder) (Variables|Default|GetTubeMaterialIndex) "/Game/Portals/Objects/ExcursionFunnel/ExcursionFunnelTubeMaterial.ExcursionFunnelTubeMaterial" "None" :!class /Script/Engine.PrimitiveComponent))
  (if Reverse
    (bind _returnvalue_2 (Rendering|Material|GetVectorParameterValue "/Game/Portals/MPC_Colors.MPC_Colors" "ExcursionFunnelTubeReverse" :!class /Script/Engine.KismetMaterialLibrary))
    (Rendering|Material|SetVectorParameterValue _returnvalue "Color" _returnvalue_2 :!class /Script/Engine.MaterialInstanceDynamic)
    (else
      (bind _returnvalue_3 (Rendering|Material|GetVectorParameterValue "/Game/Portals/MPC_Colors.MPC_Colors" "ExcursionFunnelTubeForward" :!class /Script/Engine.KismetMaterialLibrary))
      (Rendering|Material|SetVectorParameterValue _returnvalue "Color" _returnvalue_3 :!class /Script/Engine.MaterialInstanceDynamic))))