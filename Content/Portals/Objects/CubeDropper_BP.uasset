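; Portal-style cube dropper that spawns a weighted or reflective cube at its spawn point, optionally dropping one on BeginPlay.
; A drop dispatcher turns the container light orange and plays a timeline that swings both lids open.
; When fully open it spawns the cube, optionally destroying the previous one, then reverses the lids and returns the light to blue.
; Light colors come from a material parameter collection applied through dynamic material instances.
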(event Custom|DropCubeEvent
  (CallFunction|SetLightColorOrange)
  (bind (_direction _lidsdiscplacement) (Timeline|OpenLidsTimeline Play)
    (:Update
      (Transformation|SetRelativeRotation (Variables|Default|GetLeftLid) (Math|Rotator|Lerp(Rotator) "0, 0, 0" "-90.000000, 0, 0" _lidsdiscplacement) false false)
      (Transformation|SetRelativeRotation (Variables|Default|GetRightLid) (Math|Rotator|Lerp(Rotator) "0, 0, 0" "90.000000, 0, 0" _lidsdiscplacement) false false))
    (:Finished
      (if (Utilities|Enum|Equal(Enum) _direction "Forward")
        (CallFunction|DropCube)
        (Utilities|FlowControl|Delay 1.0)
        (Timeline|OpenLidsTimeline Reverse)
        (else
          (CallFunction|SetLightColorBlue))))))

(event EventBeginPlay
  (Utilities|FlowControl|Sequence
    (:then_0
      (EventDispatchers|BindEventtoDropCubeDispatcher (delegate Custom|DropCubeEvent)))
    (:then_1
      (CallFunction|SetLightColorBlue))
    (:then_2
      (if (Variables|Default|GetAutoSpawnFirstCube)
        (Default|CallDropCubeDispatcher)))))

(event Collision|EventActorBeginOverlap
  (params (OtherActor :type Actor%20Object%20Reference)))

(event EventTick
  (params (DeltaSeconds :type Float%20%28single-precision%29)))

(fn ConstructionScript)

(fn SetLightColorBlue
  (bind _returnvalue (Rendering|Material|GetVectorParameterValue "/Game/Portals/MPC_Colors.MPC_Colors" "PortalBlue" :!class /Script/Engine.KismetMaterialLibrary))
  (bind _returnvalue_2 (Rendering|Material|CreateDynamicMaterialInstance (Variables|Default|GetContainer) (Variables|Default|GetContainerLightMaterialIndex) "/Game/Portals/Models/CubeDropper/CubeDropper_Light_mat.CubeDropper_Light_mat" "None" :!class /Script/Engine.PrimitiveComponent))
  (Rendering|Material|SetVectorParameterValue _returnvalue_2 "LightColor" _returnvalue :!class /Script/Engine.MaterialInstanceDynamic))

(fn SetLightColorOrange
  (bind _returnvalue (Rendering|Material|GetVectorParameterValue "/Game/Portals/MPC_Colors.MPC_Colors" "PortalOrange" :!class /Script/Engine.KismetMaterialLibrary))
  (bind _returnvalue_2 (Rendering|Material|CreateDynamicMaterialInstance (Variables|Default|GetContainer) (Variables|Default|GetContainerLightMaterialIndex) "/Game/Portals/Models/CubeDropper/CubeDropper_Light_mat.CubeDropper_Light_mat" "None" :!class /Script/Engine.PrimitiveComponent))
  (Rendering|Material|SetVectorParameterValue _returnvalue_2 "LightColor" _returnvalue :!class /Script/Engine.MaterialInstanceDynamic))

(fn DropCube
  ;[1 1 1] Destroy LastSpawnedCube
  (if (and (Variables|Default|GetDestroyLastCubeWhenSpawningNewCube) (Utilities|IsValid (Variables|Default|GetLastSpawnedCube)))
    (Actor|DestroyActor (Variables|Default|GetLastSpawnedCube)))
  (if (== (Variables|Default|GetDroppedActor) "/Game/Portals/Objects/WeightedCube_BP.WeightedCube_BP_C")
    ;[1 1 1] Drop Weighted Cube
    (bind _returnvalue (Game|SpawnActorfromClass "/Game/Portals/Objects/WeightedCube_BP.WeightedCube_BP_C" (Math|Transform|MakeTransform (Transformation|GetWorldLocation (Variables|Default|GetCubeSpawnPoint)) "0, 0, 0" "1,1,1") "Undefined" 0 self 0))
    (Variables|Default|SetLastSpawnedCube _returnvalue)
    (elif (== (Variables|Default|GetDroppedActor) "/Game/Portals/Objects/ReflectiveCube_BP.ReflectiveCube_BP_C")
      ;[1 1 1] Drop Reflective Cube
      (bind _returnvalue_2 (Game|SpawnActorfromClass "/Game/Portals/Objects/ReflectiveCube_BP.ReflectiveCube_BP_C" (Math|Transform|MakeTransform (Transformation|GetWorldLocation (Variables|Default|GetCubeSpawnPoint)) "0, 0, 0" "1,1,1") "Undefined" 0 self 0))
      (Variables|Default|SetLastSpawnedCube _returnvalue_2))))