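; Turret actor that turns to face the first-person player and fires projectile bursts at them while enabled.
; PawnSensing sightings of a FirstPersonCharacter snap the actor's rotation toward it and trigger a burst if the Shooting flag permits.
; A ForLoopWithDelay macro spaces a random number of projectile spawns, then a random cooldown re-arms Shooting.
; An impulse-based launch remains in the graph but never runs.
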(event OnSeePawn(PawnSensing)
  (params (Pawn :type Pawn%20Object%20Reference))
  (if (Variables|Default|GetTurretEnabled)
    (bind _asfirst_person_character (Utilities|Casting|CastToFirstPersonCharacter Pawn))
    (Utilities|FlowControl|Sequence
      (:then_0
        ;[1 1 1] Rotate Turret towards player
        (bind _returnvalue (Transformation|SetActorRotation (Math|Rotator|FindLookatRotation (Transformation|GetActorLocation) (Transformation|GetActorLocation _asfirst_person_character))))
        (if (not _returnvalue)
          (Development|PrintString "Unable to set Turret rotation towards player.")))
      (:then_1
        ;[1 1 1] Shoot at player
        (if (Variables|Default|GetShooting)
          (Variables|Default|SetShooting false)
          (Utilities|ForLoopwithDelay 0 (Math|Random|RandomIntegerinRange 0 5) 0.05 ; For loop to be able to shoot in bursts.
            (:Loop%20Body
              (Game|SpawnActorfromClass "/Game/Portals/Deprecated/MyProjectile.MyProjectile_C" (Transformation|GetWorldTransform (Variables|Default|GetProjectileSpawnLocation)) "Undefined" 0 0))
            (:Completed
              (Utilities|FlowControl|Delay (Math|Random|RandomFloatinRange 0.5 2.0))
              (Variables|Default|SetShooting true))))))))

(fn ConstructionScript)