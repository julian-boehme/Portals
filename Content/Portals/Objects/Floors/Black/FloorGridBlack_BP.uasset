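; Portal level floor Blueprint that builds a tiled grid, mostly black, with white tiles marking portal-spawnable surfaces.
; The construction script loops over X and Y counts, offsetting each tile by per-axis vectors and adding it as a white or black floor instance.
; Coordinates listed in Holes are left empty, and those in PortalSpawnableSurfaces get white tiles, both found by linear search.
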(event EventBeginPlay)

(event Collision|EventActorBeginOverlap
  (params (OtherActor :type Actor%20Object%20Reference)))

(event EventTick
  (params (DeltaSeconds :type Float%20%28single-precision%29)))

(fn ConstructionScript
  ;[1 1 1] Height
  (for _index (range 0 (- (Variables|Default|GetNumAlongY) 1))
    (LocalVariables|SetCurrentYValue _index)
    (LocalVariables|SetCurrentYOffset (* (Variables|Default|GetObjectOffsetY) _index))
    ;[1 1 1] Width
    (for _index_2 (range 0 (- (Variables|Default|GetNumAlongX) 1))
      (bind _output_get (LocalVariables|SetCurrentXValue _index_2))
      (bind _ishole (CallFunction|IsHole _output_get (LocalVariables|GetCurrentYValue)))
      (if (not _ishole)
        (LocalVariables|SetSpawnLocation (+ (* (Variables|Default|GetObjectOffsetX) (LocalVariables|GetCurrentXValue)) (LocalVariables|GetCurrentYOffset)))
        (bind _isportalspawnablesurface (CallFunction|IsPortalSpawnableFloor (LocalVariables|GetCurrentXValue) (LocalVariables|GetCurrentYValue)))
        (if _isportalspawnablesurface
          (Components|InstancedStaticMesh|AddInstance (Variables|Default|GetWhiteFloor) (Math|Transform|MakeTransform (LocalVariables|GetSpawnLocation) "0, 0, 0" "1,1,1"))
          (else
            (Components|InstancedStaticMesh|AddInstance (Variables|Default|GetBlackFloor) (Math|Transform|MakeTransform (LocalVariables|GetSpawnLocation) "0, 0, 0" "1,1,1"))))))))

(fn IsPortalSpawnableFloor
  (params (X :type Integer) (Y :type Integer))
  (for _array_element (Variables|Default|GetPortalSpawnableSurfaces)
    (if (and (== (.X (Math|Vector|BreakVector _array_element)) (Math|Conversions|ToFloat(Integer) X)) (== (.Y (Math|Vector|BreakVector _array_element)) (Math|Conversions|ToFloat(Integer) Y)))
      (return true)))
  (return false))

(fn IsHole
  (params (X :type Integer) (Y :type Integer))
  (for _array_element (Variables|Default|GetHoles)
    (if (and (== (.X (Math|Vector|BreakVector _array_element)) (Math|Conversions|ToFloat(Integer) X)) (== (.Y (Math|Vector|BreakVector _array_element)) (Math|Conversions|ToFloat(Integer) Y)))
      (return true)))
  (return false))