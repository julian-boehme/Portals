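; Lift platform that travels between a start and end point, optionally triggered by the player standing on it.
; A timeline, rate-scaled by MovementSpeed, lerps the platform, reversing after a wait at the end or when the player steps off.
; Enabled gates player-triggered departure and sets the light color from a material parameter collection.
; The construction script positions the platform and a destination preview hidden in game.
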(event OnComponentBeginOverlap(Box)
  (params (OverlappedComponent :type Primitive%20Component%20Object%20Reference) (OtherActor :type Actor%20Object%20Reference) (OtherComp :type Primitive%20Component%20Object%20Reference) (OtherBodyIndex :type Integer) (bFromSweep :type Boolean) (SweepResult :type Hit%20Result%20Structure%20%28by%20ref%29))
  ;[1 1 1] Player stepped on platform
  (if (Variables|Default|GetMoveWhenPlayerSteppedOn)
    (Utilities|Casting|CastToFirstPersonCharacter OtherActor)
    (if (Variables|Default|GetEnabled)
      (Audio|Components|Audio|Play (Variables|Default|GetTimeline_0)))))

(event OnComponentEndOverlap(Box)
  (params (OverlappedComponent :type Primitive%20Component%20Object%20Reference) (OtherActor :type Actor%20Object%20Reference) (OtherComp :type Primitive%20Component%20Object%20Reference) (OtherBodyIndex :type Integer))
  ;[1 1 1] Player left platform
  (if (Variables|Default|GetMoveWhenPlayerSteppedOn)
    (Utilities|Casting|CastToFirstPersonCharacter OtherActor)
    (Utilities|String|Reverse (Variables|Default|GetTimeline_0))))

(event EventBeginPlay
  ;[1 1 1] Apply movementSpeed by setting the PlayRate of the Timeline
  (Components|Timeline|SetPlayRate (Variables|Default|GetTimeline_0) (Variables|Default|GetMovementSpeed)))

(event Collision|EventActorBeginOverlap
  (params (OtherActor :type Actor%20Object%20Reference)))

(event EventTick
  (params (DeltaSeconds :type Float%20%28single-precision%29)))

(fn ConstructionScript
  (if (Variables|Default|GetEnabled)
    (CallFunction|SetLighttoActivatedColor)
    (else
      (CallFunction|SetLighttoDeactivatedColor)))
  ;[1 1 1] Needs to be set here. Once I defined a constructor for this object, the "Hidden In Game" option in the "Details" panel doesn't work anymore.
  (Development|SetHiddeninGame (Variables|Default|GetDestinationPreview) true true)
  ;[1 1 1] Position platform at StartPoint
  (Transformation|SetRelativeLocation (Variables|Default|GetLift) (Variables|Default|GetStartPoint) false false)
  ;[1 1 1] Position destination preview
  (Transformation|SetRelativeLocation (Variables|Default|GetDestinationPreview) (Variables|Default|GetEndPoint) false false))

(fn SetEnabled
  (params (Enabled :type Boolean))
  (bind _output_get (Variables|Default|SetEnabled Enabled))
  (if _output_get
    (CallFunction|SetLighttoActivatedColor)
    (else
      (CallFunction|SetLighttoDeactivatedColor))))

(fn SetLighttoActivatedColor
  (bind _returnvalue (Rendering|Material|GetVectorParameterValue "/Game/Portals/MPC_Colors.MPC_Colors" "LiftActivatedColor" :!class /Script/Engine.KismetMaterialLibrary))
  (bind _returnvalue_2 (Rendering|Material|CreateDynamicMaterialInstance (Variables|Default|GetLift) (LocalVariables|GetLiftLightMaterialIndex) "/Game/Portals/Models/Lift/LiftLight_mat.LiftLight_mat" "None" :!class /Script/Engine.PrimitiveComponent))
  (Rendering|Material|SetVectorParameterValue _returnvalue_2 "LightColor" _returnvalue :!class /Script/Engine.MaterialInstanceDynamic))

(fn SetLighttoDeactivatedColor
  (bind _returnvalue (Rendering|Material|GetVectorParameterValue "/Game/Portals/MPC_Colors.MPC_Colors" "LiftDeactivatedColor" :!class /Script/Engine.KismetMaterialLibrary))
  (bind _returnvalue_2 (Rendering|Material|CreateDynamicMaterialInstance (Variables|Default|GetLift) (LocalVariables|GetLiftLightMaterialIndex) "/Game/Portals/Models/Lift/LiftLight_mat.LiftLight_mat" "None" :!class /Script/Engine.PrimitiveComponent))
  (Rendering|Material|SetVectorParameterValue _returnvalue_2 "LightColor" _returnvalue :!class /Script/Engine.MaterialInstanceDynamic))