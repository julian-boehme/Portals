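; SuperButton is a floor-button style actor for the portals game, pressed while the player or a physics body overlaps its Box.
; Overlap begin and end set the pressed state, fire OnPressedStatusChanged, and play or reverse a timeline that slides the plate.
; When the timeline finishes, it recolors the base light and any overlapped WeightedCube from a material parameter collection.
; Only the last entering actor is tracked, and any qualifying exit releases the button.
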(event OnComponentBeginOverlap(Box)
  (params (OverlappedComponent :type Primitive%20Component%20Object%20Reference) (OtherActor :type Actor%20Object%20Reference) (OtherComp :type Primitive%20Component%20Object%20Reference) (OtherBodyIndex :type Integer) (bFromSweep :type Boolean) (SweepResult :type Hit%20Result%20Structure%20%28by%20ref%29))
  (bind _isplayerorphysicsbody (CallFunction|IsPlayerorPhysicsBody OtherActor))
  (if _isplayerorphysicsbody
    (Variables|Default|SetOverlappedActor OtherActor)
    (CallFunction|SetIsPressed true)
    (bind (_direction _buttondisplacement) (Timeline|PressedTimeline Play)
      (:Update
        (Transformation|SetRelativeLocation (Variables|Default|GetButton%20Plate) (Math|Vector|Lerp(Vector) (Variables|Default|GetButtonUnpressedLocation) (Variables|Default|GetButtonPressedLocation) _buttondisplacement) false false))
      (:Finished
        ;[1 1 1] Change material colors of ButtonBase and WeightedCube
        (if (Utilities|Enum|Equal(Enum) _direction "Forward")
          ;;[1 1 1] Pressed
          (bind _returnvalue (Rendering|Material|CreateDynamicMaterialInstance (Variables|Default|GetButton%20Base) (Variables|Default|GetActivationLightMaterialIndex) "/Game/Portals/Models/SuperButton/SuperButtonActivationLight_mat.SuperButtonActivationLight_mat" "None" :!class /Script/Engine.PrimitiveComponent))
          (bind _returnvalue_2 (Rendering|Material|GetVectorParameterValue "/Game/Portals/MPC_Colors.MPC_Colors" "SuperButtonActivatedColor" :!class /Script/Engine.KismetMaterialLibrary))
          (Rendering|Material|SetVectorParameterValue _returnvalue "ActivationLight" _returnvalue_2 :!class /Script/Engine.MaterialInstanceDynamic)
          (bind _asweighted_cube_bp (Utilities|Casting|CastToWeightedCube_BP (Variables|Default|GetOverlappedActor)))
          (bind _returnvalue_3 (Rendering|Material|GetVectorParameterValue "/Game/Portals/MPC_Colors.MPC_Colors" "CubeActivatedColor" :!class /Script/Engine.KismetMaterialLibrary))
          (Default|SetCircleColor _asweighted_cube_bp _returnvalue_3)
          (else
            ;;[1 1 1] Not Pressed
            (bind _returnvalue_4 (Rendering|Material|CreateDynamicMaterialInstance (Variables|Default|GetButton%20Base) (Variables|Default|GetActivationLightMaterialIndex) "/Game/Portals/Models/SuperButton/SuperButtonActivationLight_mat.SuperButtonActivationLight_mat" "None" :!class /Script/Engine.PrimitiveComponent))
            (bind _returnvalue_5 (Rendering|Material|GetVectorParameterValue "/Game/Portals/MPC_Colors.MPC_Colors" "SuperButtonDeactivatedColor" :!class /Script/Engine.KismetMaterialLibrary))
            (Rendering|Material|SetVectorParameterValue _returnvalue_4 "ActivationLight" _returnvalue_5 :!class /Script/Engine.MaterialInstanceDynamic)
            (bind _asweighted_cube_bp_2 (Utilities|Casting|CastToWeightedCube_BP (Variables|Default|GetOverlappedActor)))
            (bind _returnvalue_6 (Rendering|Material|GetVectorParameterValue "/Game/Portals/MPC_Colors.MPC_Colors" "CubeDeactivatedColor" :!class /Script/Engine.KismetMaterialLibrary))
            (Default|SetCircleColor _asweighted_cube_bp_2 _returnvalue_6)))))))

(event OnComponentEndOverlap(Box)
  (params (OverlappedComponent :type Primitive%20Component%20Object%20Reference) (OtherActor :type Actor%20Object%20Reference) (OtherComp :type Primitive%20Component%20Object%20Reference) (OtherBodyIndex :type Integer))
  (bind _isplayerorphysicsbody (CallFunction|IsPlayerorPhysicsBody OtherActor))
  (if _isplayerorphysicsbody
    (CallFunction|SetIsPressed false)
    (bind (_direction _buttondisplacement) (Timeline|PressedTimeline Reverse)
      (:Update
        (Transformation|SetRelativeLocation (Variables|Default|GetButton%20Plate) (Math|Vector|Lerp(Vector) (Variables|Default|GetButtonUnpressedLocation) (Variables|Default|GetButtonPressedLocation) _buttondisplacement) false false))
      (:Finished
        ;[1 1 1] Change material colors of ButtonBase and WeightedCube
        (if (Utilities|Enum|Equal(Enum) _direction "Forward")
          ;;[1 1 1] Pressed
          (bind _returnvalue (Rendering|Material|CreateDynamicMaterialInstance (Variables|Default|GetButton%20Base) (Variables|Default|GetActivationLightMaterialIndex) "/Game/Portals/Models/SuperButton/SuperButtonActivationLight_mat.SuperButtonActivationLight_mat" "None" :!class /Script/Engine.PrimitiveComponent))
          (bind _returnvalue_2 (Rendering|Material|GetVectorParameterValue "/Game/Portals/MPC_Colors.MPC_Colors" "SuperButtonActivatedColor" :!class /Script/Engine.KismetMaterialLibrary))
          (Rendering|Material|SetVectorParameterValue _returnvalue "ActivationLight" _returnvalue_2 :!class /Script/Engine.MaterialInstanceDynamic)
          (bind _asweighted_cube_bp (Utilities|Casting|CastToWeightedCube_BP (Variables|Default|GetOverlappedActor)))
          (bind _returnvalue_3 (Rendering|Material|GetVectorParameterValue "/Game/Portals/MPC_Colors.MPC_Colors" "CubeActivatedColor" :!class /Script/Engine.KismetMaterialLibrary))
          (Default|SetCircleColor _asweighted_cube_bp _returnvalue_3)
          (else
            ;;[1 1 1] Not Pressed
            (bind _returnvalue_4 (Rendering|Material|CreateDynamicMaterialInstance (Variables|Default|GetButton%20Base) (Variables|Default|GetActivationLightMaterialIndex) "/Game/Portals/Models/SuperButton/SuperButtonActivationLight_mat.SuperButtonActivationLight_mat" "None" :!class /Script/Engine.PrimitiveComponent))
            (bind _returnvalue_5 (Rendering|Material|GetVectorParameterValue "/Game/Portals/MPC_Colors.MPC_Colors" "SuperButtonDeactivatedColor" :!class /Script/Engine.KismetMaterialLibrary))
            (Rendering|Material|SetVectorParameterValue _returnvalue_4 "ActivationLight" _returnvalue_5 :!class /Script/Engine.MaterialInstanceDynamic)
            (bind _asweighted_cube_bp_2 (Utilities|Casting|CastToWeightedCube_BP (Variables|Default|GetOverlappedActor)))
            (bind _returnvalue_6 (Rendering|Material|GetVectorParameterValue "/Game/Portals/MPC_Colors.MPC_Colors" "CubeDeactivatedColor" :!class /Script/Engine.KismetMaterialLibrary))
            (Default|SetCircleColor _asweighted_cube_bp_2 _returnvalue_6)))))))

(event EventBeginPlay)

(event Collision|EventActorBeginOverlap
  (params (OtherActor :type Actor%20Object%20Reference)))

(event EventTick
  (params (DeltaSeconds :type Float%20%28single-precision%29)))

(fn ConstructionScript)

(fn SetIsPressed
  (params (Pressed :type Boolean))
  (bind _output_get (Variables|Default|SetPressed Pressed))
  (Default|CallOnPressedStatusChanged _output_get))

(fn IsPlayerorPhysicsBody
  (params (Actor :type Actor%20Object%20Reference))
  (Utilities|Casting|CastToFirstPersonCharacter Actor
    (:then
      (return true))
    (:CastFailed
      (if (Utilities|Enum|Equal(Enum) (Collision|GetCollisionObjectType (Actor|GetComponentbyClass Actor "/Script/Engine.PrimitiveComponent")) "ECC_PhysicsBody")
        (return true)
        (else
          (return false))))))