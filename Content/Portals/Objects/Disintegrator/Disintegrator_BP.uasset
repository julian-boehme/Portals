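; Disintegrator gate for the portal game: the player passing through hides both portals, and any other overlapping actor is destroyed.
; The Construction Script positions two posts along local X and, when enabled, stretches and centers the Sensor volume between them.
; Sensor overlap drives the effect only while Enabled, finding the Portal A and B actors by class.
; SetEnabled toggles that flag along with the Sensor's visibility.
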(event OnComponentBeginOverlap(Sensor)
  (params (OverlappedComponent :type Primitive%20Component%20Object%20Reference) (OtherActor :type Actor%20Object%20Reference) (OtherComp :type Primitive%20Component%20Object%20Reference) (OtherBodyIndex :type Integer) (bFromSweep :type Boolean) (SweepResult :type Hit%20Result%20Structure%20%28by%20ref%29))
  (if (Variables|Default|GetEnabled)
    (Utilities|Casting|CastToFirstPersonCharacter OtherActor
      (:then
        (Development|PrintString "Destroying Portals")
        (Utilities|FlowControl|Sequence
          (:then_0
            (bind _returnvalue (Actor|GetActorOfClass "/Game/Portals/Objects/Portals/Portal_A_BP_Child.Portal_A_BP_Child_C"))
            (Default|SetPortalVisibility _returnvalue false))
          (:then_1
            (bind _returnvalue_2 (Actor|GetActorOfClass "/Game/Portals/Objects/Portals/Portal_B_BP_Child.Portal_B_BP_Child_C"))
            (Default|SetPortalVisibility _returnvalue_2 false))))
      (:CastFailed
        (Actor|DestroyActor OtherActor)))))

(event EventBeginPlay)

(event Collision|EventActorBeginOverlap
  (params (OtherActor :type Actor%20Object%20Reference)))

(event EventTick
  (params (DeltaSeconds :type Float%20%28single-precision%29)))

(fn ConstructionScript
  (bind _right_post (Variables|Default|GetRight%20Post))
  (bind _left_post (Variables|Default|GetLeft%20Post))
  (bind _sensor (Variables|Default|GetSensor))
  (bind _sensor_2 (Variables|Default|GetSensor))
  (bind _rightpostlocation (Variables|Default|GetRightPostLocation))
  (bind _leftpostlocation (Variables|Default|GetLeftPostLocation))
  (bind _returnvalue (- _rightpostlocation _leftpostlocation))
  (bind _relativelocation (Variables|/Script/Engine.SceneComponent|GetRelativeLocation _right_post))
  (bind _relativelocation_2 (Variables|/Script/Engine.SceneComponent|GetRelativeLocation _left_post))
  (bind _relativelocation_3 (Variables|/Script/Engine.SceneComponent|GetRelativeLocation _sensor_2))
  (bind _relativescale3d (Variables|/Script/Engine.SceneComponent|GetRelativeScale3D _sensor))
  (Transformation|SetRelativeLocation _left_post (Math|Vector|MakeVector (.x (Variables|Default|GetLeftPostLocation)) (.y _relativelocation_2) (.z _relativelocation_2)) false false)
  (Transformation|SetRelativeLocation _right_post (Math|Vector|MakeVector (.x (Variables|Default|GetRightPostLocation)) (.y _relativelocation) (.z _relativelocation)) false false)
  (if (Variables|Default|GetEnabled)
    ;[1 1 1] Scale sensor to fill area between posts.
    (Transformation|SetRelativeScale3D _sensor (Math|Vector|MakeVector (/ (.X (Math|Vector|BreakVector _returnvalue)) 1e+02) (.y _relativescale3d) (.z _relativescale3d)))
    (Transformation|SetRelativeLocation _sensor_2 (Math|Vector|MakeVector (.x (+ _leftpostlocation (/ _returnvalue 2))) (.y _relativelocation_3) (.z _relativelocation_3)) false false)
    (else
      (Rendering|SetVisibility (Variables|Default|GetSensor) false false))))

(fn SetEnabled
  (params (Enabled :type Boolean))
  (bind _output_get (Variables|Default|SetEnabled Enabled))
  (Rendering|SetVisibility (Variables|Default|GetSensor) _output_get false))