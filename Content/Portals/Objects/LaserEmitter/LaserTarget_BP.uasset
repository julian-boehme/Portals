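; Laser target actor that detects when a laser hits it and reports changes in its hit status.
; Begin and end overlaps between its model and a Laser_BP actor call SetHit, which stores the state and fires the HitStatusChanged dispatcher.
; SetHit also recolors the target's light, creating a new dynamic material instance on each call with hit or not-hit colors from the MPC_Colors parameter collection.
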(event OnComponentBeginOverlap(LaserTargetModel)
  (params (OverlappedComponent :type Primitive%20Component%20Object%20Reference) (OtherActor :type Actor%20Object%20Reference) (OtherComp :type Primitive%20Component%20Object%20Reference) (OtherBodyIndex :type Integer) (bFromSweep :type Boolean) (SweepResult :type Hit%20Result%20Structure%20%28by%20ref%29))
  (Utilities|Casting|CastToLaser_BP OtherActor)
  (CallFunction|SetHit true))

(event OnComponentEndOverlap(LaserTargetModel)
  (params (OverlappedComponent :type Primitive%20Component%20Object%20Reference) (OtherActor :type Actor%20Object%20Reference) (OtherComp :type Primitive%20Component%20Object%20Reference) (OtherBodyIndex :type Integer))
  (Utilities|Casting|CastToLaser_BP OtherActor)
  (CallFunction|SetHit false))

(event EventBeginPlay)

(event Collision|EventActorBeginOverlap
  (params (OtherActor :type Actor%20Object%20Reference)))

(event EventTick
  (params (DeltaSeconds :type Float%20%28single-precision%29)))

(fn ConstructionScript)

(fn SetHit
  (params (IsHit :type Boolean))
  (bind _output_get (Variables|Default|SetHit IsHit))
  (if _output_get
    (bind _returnvalue (Rendering|Material|CreateDynamicMaterialInstance (Variables|Default|GetLaserTargetModel) (Variables|Default|GetLaserTargetRedLightMaterialIndex) "/Game/Portals/Models/LaserTarget/LaserTarget_RedLight_mat.LaserTarget_RedLight_mat" "None" :!class /Script/Engine.PrimitiveComponent))
    (bind _returnvalue_2 (Rendering|Material|GetVectorParameterValue "/Game/Portals/MPC_Colors.MPC_Colors" "LaserTargetHitColor" :!class /Script/Engine.KismetMaterialLibrary))
    (Rendering|Material|SetVectorParameterValue _returnvalue "LightColor" _returnvalue_2 :!class /Script/Engine.MaterialInstanceDynamic)
    (else
      (bind _returnvalue_3 (Rendering|Material|CreateDynamicMaterialInstance (Variables|Default|GetLaserTargetModel) (Variables|Default|GetLaserTargetRedLightMaterialIndex) "/Game/Portals/Models/LaserTarget/LaserTarget_RedLight_mat.LaserTarget_RedLight_mat" "None" :!class /Script/Engine.PrimitiveComponent))
      (bind _returnvalue_4 (Rendering|Material|GetVectorParameterValue "/Game/Portals/MPC_Colors.MPC_Colors" "LaserTargetNotHitColor" :!class /Script/Engine.KismetMaterialLibrary))
      (Rendering|Material|SetVectorParameterValue _returnvalue_3 "LightColor" _returnvalue_4 :!class /Script/Engine.MaterialInstanceDynamic)))
  (Default|CallHitStatusChanged _output_get))