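; Laser emitter for portal puzzles that fires a beam which reflects off cubes, passes through portals and hits laser targets.
; BeginPlay spawns a hidden pool of Laser_BP segments and binds to its targets, broadcasting whether all are hit whenever one changes.
; While enabled, Tick hides the segments and runs a recursive, count-capped line trace, stretching one segment per hop.
; Reflective cubes redirect the trace, active portal pairs convert it, and pass-through targets continue it.
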(event Custom|HitStatusChanged_Event_0
  (params (IsHit :type Boolean))
  ;[1 1 1] Bind lasers
  (bind _allhit (CallFunction|AllLaserTargetsHit))
  (Default|CallAllLaserHitStatusChanged _allhit))

(event EventBeginPlay
  ;[1 1 1] Setup laser array
  (for _index (range 0 (- (Variables|Default|GetMaxNumOfLasers) 1))
    (bind _returnvalue (Game|SpawnActorfromClass "/Game/Portals/Objects/LaserEmitter/Laser_BP.Laser_BP_C" (Math|Transform|MakeTransform "0, 0, 0" "0, 0, 0" "1,1,1") "Undefined" 0 "-500.000000,0.000000,0.000000" "500.000000,0.000000,0.000000" self 0))
    (Default|SetLaserVisibility _returnvalue false)
    (Utilities|Array|Add (Variables|Default|GetLaserBeams) _returnvalue)
    ;[1 1 1] Bind lasers
    (for _array_element (Variables|Default|GetLaserTargets)
      (EventDispatchers|AssignHitStatusChanged _array_element (delegate Custom|HitStatusChanged_Event_0)))))

(event Collision|EventActorBeginOverlap
  (params (OtherActor :type Actor%20Object%20Reference)))

(event EventTick
  (params (DeltaSeconds :type Float%20%28single-precision%29))
  (if (Variables|Default|GetEnabled)
    (CallFunction|UpdateLasers)))

(fn ConstructionScript)

(fn MakeLineTrace
  (params (Start :type Vector) (Direction :type Vector) (CurrentTraceNr :type Integer) (IgnoredActor :type Actor%20Object%20Reference))
  ;[1 1 1] Make line-trace
  (if (< CurrentTraceNr (Variables|Default|GetMaxNumOfLasers))
    (bind _output_get (LocalVariables|SetEnd (+ Start (* Direction (Variables|Default|GetMaxTraceDistance)))))
    (bind (_outhit _returnvalue) (Collision|LineTraceByChannel Start _output_get "TraceTypeQuery3" false (Utilities|Array|MakeArray IgnoredActor) "None"))
    (if _returnvalue
      (LocalVariables|SetHit%20Location (.Location (Collision|BreakHitResult _outhit)))
      (LocalVariables|SetHitActor (.HitActor (Collision|BreakHitResult _outhit)))
      ;[1 1 1] Extend laser to the hit object.
      (CallFunction|ExtendLaser Start (LocalVariables|GetHit%20Location) CurrentTraceNr)
      ;[1 1 1] If hit actor is ReflectorCube, make another line-trace
      (bind _asreflective_cube_bp (Utilities|Casting|CastToReflectiveCube_BP (LocalVariables|GetHitActor))
        (:then
          (Variables|/Game/Portals/Objects/ReflectiveCube_BP.ReflectiveCube_BP_C|SetLaserEmitter _asreflective_cube_bp self)
          (CallFunction|MakeLineTrace (Transformation|GetActorLocation _asreflective_cube_bp) (Math|Vector|GetForwardVector (Variables|/Game/Portals/Objects/ReflectiveCube_BP.ReflectiveCube_BP_C|GetCube _asreflective_cube_bp)) (+ CurrentTraceNr 1) _asreflective_cube_bp))
        (:CastFailed
          ;[1 1 1] Hit Portal A
          (bind _asportal_a_bp_child (Utilities|Casting|CastToPortal_A_BP_Child (LocalVariables|GetHitActor))
            (:then
              (bind _canteleport (CallFunction|PortalsCanTeleport))
              (if _canteleport
                (bind _returnvalue_2 (Actor|GetActorOfClass "/Game/Portals/Objects/Portals/Portal_B_BP_Child.Portal_B_BP_Child_C"))
                (bind _newlocation (Default|UConvertLocation _returnvalue_2 _asportal_a_bp_child _returnvalue_2 (LocalVariables|GetHit%20Location) false false false 0.0))
                (bind _newdirection (Default|UConvertDirection _asportal_a_bp_child _asportal_a_bp_child _returnvalue_2 Direction))
                (CallFunction|MakeLineTrace _newlocation _newdirection (+ CurrentTraceNr 1) _returnvalue_2)))
            (:CastFailed
              ;[1 1 1] Hit Portal B
              (bind _asportal_b_bp_child (Utilities|Casting|CastToPortal_B_BP_Child (LocalVariables|GetHitActor))
                (:then
                  (bind _canteleport_2 (CallFunction|PortalsCanTeleport))
                  (if _canteleport_2
                    (bind _returnvalue_3 (Actor|GetActorOfClass "/Game/Portals/Objects/Portals/Portal_A_BP_Child.Portal_A_BP_Child_C"))
                    (bind _newlocation_2 (Default|UConvertLocation _returnvalue_3 _asportal_b_bp_child _returnvalue_3 (LocalVariables|GetHit%20Location) false false false 0.0))
                    (bind _newdirection_2 (Default|UConvertDirection _asportal_b_bp_child _asportal_b_bp_child _returnvalue_3 Direction))
                    (CallFunction|MakeLineTrace _newlocation_2 _newdirection_2 (+ CurrentTraceNr 1) _returnvalue_3)))
                (:CastFailed
                  ;[1 1 1] Hit Laser Target
                  (bind _aslaser_target_bp (Utilities|Casting|CastToLaserTarget_BP (LocalVariables|GetHitActor)))
                  ;;[1 1 1] Extend laser to Laser Target
                  (CallFunction|ExtendLaser Start (LocalVariables|GetHit%20Location) CurrentTraceNr)
                  (if (Variables|/Game/Portals/Objects/LaserEmitter/LaserTarget_BP.LaserTarget_BP_C|GetIsPassThrough _aslaser_target_bp)
                    ;;[1 1 1] Make another line-trace behind the object.
                    (CallFunction|MakeLineTrace (LocalVariables|GetHit%20Location) Direction (+ CurrentTraceNr 1) _aslaser_target_bp))))))))
      (else
        ;[1 1 1] Extend Laser to maximum length
        (CallFunction|ExtendLaser Start (LocalVariables|GetEnd) CurrentTraceNr)))))

(fn UpdateLasers
  (for _array_element (Variables|Default|GetLaserBeams)
    (Default|SetLaserVisibility _array_element false))
  (CallFunction|MakeLineTrace (Transformation|GetWorldLocation (Variables|Default|GetLaserStartPoint)) (Math|Vector|GetForwardVector (Variables|Default|GetArrow))))

(fn ExtendLaser
  (params (Start :type Vector) (End :type Vector) (CurrentTraceNr :type Integer))
  (bind _laserbeams (Variables|Default|GetLaserBeams))
  (bind _output (Utilities|Array|Get(acopy) _laserbeams CurrentTraceNr))
  (Default|SetLaserVisibility _output true)
  (Variables|/Game/Portals/Objects/LaserEmitter/Laser_BP.Laser_BP_C|SetStartPoint _output Start)
  (Variables|/Game/Portals/Objects/LaserEmitter/Laser_BP.Laser_BP_C|SetEndPoint _output End)
  (Default|CalculateLaser _output)
  (Utilities|Array|SetArrayElem _laserbeams CurrentTraceNr _output))

(fn ExtendLasertoHitObject
  (params (Start :type Vector) (HitLocation :type Vector) (CurrentTraceNr :type Integer))
  (bind _laserbeams (Variables|Default|GetLaserBeams))
  (bind _output (Utilities|Array|Get(acopy) _laserbeams CurrentTraceNr))
  (Default|SetLaserVisibility _output true)
  (Variables|/Game/Portals/Objects/LaserEmitter/Laser_BP.Laser_BP_C|SetStartPoint _output Start)
  (Variables|/Game/Portals/Objects/LaserEmitter/Laser_BP.Laser_BP_C|SetEndPoint _output HitLocation)
  (Default|CalculateLaser _output)
  (Utilities|Array|SetArrayElem _laserbeams CurrentTraceNr _output))

(fn SetEnabled
  (params (Enabled :type Boolean))
  (bind _output_get (Variables|Default|SetEnabled Enabled))
  (if (not _output_get)
    (for _array_element (Variables|Default|GetLaserBeams)
      (Default|SetLaserVisibility _array_element false))))

(fn AllLaserTargetsHit
  (for _array_element (Variables|Default|GetLaserTargets)
    (if (not (Variables|/Game/Portals/Objects/LaserEmitter/LaserTarget_BP.LaserTarget_BP_C|GetHit _array_element))
      (return false)))
  (return true))

(fn PortalsCanTeleport
  (bind _returnvalue (Actor|GetActorOfClass "/Game/Portals/Objects/Portals/Portal_A_BP_Child.Portal_A_BP_Child_C"))
  (Utilities|IsValid _returnvalue
    (:Is%20Valid
      (bind _returnvalue_2 (Actor|GetActorOfClass "/Game/Portals/Objects/Portals/Portal_B_BP_Child.Portal_B_BP_Child_C"))
      (Utilities|IsValid _returnvalue_2
        (:Is%20Valid
          (bind _visible (Default|GetPortalVisibility _returnvalue))
          (bind _visible_2 (Default|GetPortalVisibility _returnvalue_2))
          (return (Math|Boolean|ANDBoolean _visible _visible_2 (Variables|/Game/Portals/Objects/Portals/PortalSuperclass.PortalSuperclass_C|GetCanTeleport _returnvalue_2) (Variables|/Game/Portals/Objects/Portals/PortalSuperclass.PortalSuperclass_C|GetCanTeleport _returnvalue))))))))