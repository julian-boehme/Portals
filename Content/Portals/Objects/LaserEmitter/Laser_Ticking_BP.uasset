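; Laser beam segment actor for the portals laser emitter, drawn as a cylinder stretched between a start point and an end point.
; On construction, CalculateLaser turns off overlap listening, aims the cylinder's Z axis along the beam and scales its length by a distance conversion value.
; When listening is enabled, cylinder begin and end overlaps print a debug message and tell the owning LaserEmitter to update its lasers.
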(event OnComponentBeginOverlap(Cylinder)
  (params (OverlappedComponent :type Primitive%20Component%20Object%20Reference) (OtherActor :type Actor%20Object%20Reference) (OtherComp :type Primitive%20Component%20Object%20Reference) (OtherBodyIndex :type Integer) (bFromSweep :type Boolean) (SweepResult :type Hit%20Result%20Structure%20%28by%20ref%29))
  (if (Variables|Default|GetListenForOverlap)
    (Development|PrintString "HIT")
    (Default|UpdateLasers (Variables|Default|GetLaserEmitter))))

(event OnComponentEndOverlap(Cylinder)
  (params (OverlappedComponent :type Primitive%20Component%20Object%20Reference) (OtherActor :type Actor%20Object%20Reference) (OtherComp :type Primitive%20Component%20Object%20Reference) (OtherBodyIndex :type Integer))
  (if (Variables|Default|GetListenForOverlap)
    (Development|PrintString "HIT")
    (Default|UpdateLasers (Variables|Default|GetLaserEmitter))))

(event EventBeginPlay)

(event Collision|EventActorBeginOverlap
  (params (OtherActor :type Actor%20Object%20Reference)))

(event EventTick
  (params (DeltaSeconds :type Float%20%28single-precision%29)))

(fn ConstructionScript
  (CallFunction|CalculateLaser))

(fn CalculateLaser
  (bind _cylinder (Variables|Default|GetCylinder))
  (bind _startpoint (Variables|Default|GetStartPoint))
  (bind _endpoint (Variables|Default|GetEndPoint))
  (bind _returnvalue (- _endpoint _startpoint))
  (bind _relativescale3d (Variables|/Script/Engine.SceneComponent|GetRelativeScale3D _cylinder))
  (Variables|Default|SetListenForOverlap false)
  ;[1 1 1] Rotate laser
  (Transformation|SetRelativeRotation (Variables|Default|GetCylinder) (Math|Rotator|MakeRotfromZ _returnvalue) false false)
  ;[1 1 1] Scale laser
  (Transformation|SetRelativeScale3D _cylinder (Math|Vector|MakeVector (.x _relativescale3d) (.y _relativescale3d) (/ (Math|Vector|VectorLength _returnvalue) (Variables|Default|GetDistanceToScaleConversionValue)))))