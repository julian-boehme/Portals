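; Light bridge emitter that, if enabled, spawns a LightBridgeSurface actor on BeginPlay along its arrow direction.
; SetSurfaceLocationAndScale line-traces to the first blocking object, then centers and X-scales the surface to that distance, or to a maximum length on a miss.
; Visibility changes on either portal destroy the secondary SurfaceB, which is not spawned here.
; The player's portal-spawning event is bound to an empty handler.
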(event Custom|OnPortalVisibilityBChanged
  (bind _surfaceb (Variables|Default|GetSurfaceB))
  (bind _cube (Variables|/Game/Portals/Objects/LightBridge/LightBridgeSurface_BP.LightBridgeSurface_BP_C|GetCube _surfaceb))
  ;[1 1 1] Bind Event Portal OnSetVisible
  ;[1 1 1] Remove SurfaceB if Portal location is changing.
  (Utilities|IsValid _surfaceb
    (:Is%20Valid
      (Development|PrintString "Removing Surface B" true true "(R=0.170000,G=0.100721,B=1.000000,A=1.000000)")
      (Collision|SetCollisionEnabled _cube "NoCollision")
      (Rendering|SetVisibility _cube false false)
      (Actor|DestroyActor _surfaceb))))

(event Custom|OnPortalSpawning
  ;[1 1 1] Bind Event Portal OnPortalSpawning
)

(event Custom|OnPortalVisibilityAChanged
  (bind _surfaceb (Variables|Default|GetSurfaceB))
  (bind _cube (Variables|/Game/Portals/Objects/LightBridge/LightBridgeSurface_BP.LightBridgeSurface_BP_C|GetCube _surfaceb))
  ;[1 1 1] Bind Event Portal OnSetVisible
  ;[1 1 1] Remove SurfaceB if Portal location is changing.
  (Utilities|IsValid _surfaceb
    (:Is%20Valid
      (Development|PrintString "Removing Surface B" true true "(R=0.170000,G=0.100721,B=1.000000,A=1.000000)")
      (Collision|SetCollisionEnabled _cube "NoCollision")
      (Rendering|SetVisibility _cube false false)
      (Actor|DestroyActor _surfaceb))))

(event EventBeginPlay
  (if (Variables|Default|GetEnabled)
    (bind _returnvalue (Game|SpawnActorfromClass "/Game/Portals/Objects/LightBridge/LightBridgeSurface_BP.LightBridgeSurface_BP_C" (Math|Transform|MakeTransform "0, 0, 0" (Transformation|GetActorRotation) "1,1,1") "Undefined" 0 self 0))
    (bind _output_get (Variables|Default|SetSurfaceA _returnvalue))
    (CallFunction|SetSurfaceLocationandScale _output_get (Transformation|GetWorldLocation (Variables|Default|GetSurfaceLineTraceStart)) (Math|Vector|GetForwardVector (Variables|Default|GetArrow1)))
    (Utilities|FlowControl|Sequence
      (:then_0
        ;[1 1 1] Bind Event Portal OnSetVisible
        (EventDispatchers|BindEventtoOnSetVisible (Variables|Default|GetPortalA) (delegate Custom|OnPortalVisibilityAChanged)))
      (:then_1
        ;[1 1 1] Bind Event Portal OnSetVisible
        (EventDispatchers|BindEventtoOnSetVisible (Variables|Default|GetPortalB) (delegate Custom|OnPortalVisibilityBChanged)))
      (:then_2
        ;[1 1 1] Bind Event Portal OnPortalSpawning
        (bind _asfirst_person_character (Utilities|Casting|CastToFirstPersonCharacter (Game|GetPlayerCharacter 0)))
        (EventDispatchers|BindEventtoPortalSpawning _asfirst_person_character (delegate Custom|OnPortalSpawning))))))

(event Collision|EventActorBeginOverlap
  (params (OtherActor :type Actor%20Object%20Reference)))

(event EventTick
  (params (DeltaSeconds :type Float%20%28single-precision%29)))

(fn ConstructionScript)

(fn SetSurfaceLocationandScale
  (params (Surface :type Light%20Bridge%20Surface%20BP%20Object%20Reference) (StartLocation :type Vector) (TraceDirection :type Vector))
  (LocalVariables|SetSurfaveVar Surface)
  (LocalVariables|SetStartLocationVar StartLocation)
  (bind _output_get (LocalVariables|SetTraceDirectionVar TraceDirection))
  ;[1 1 1] Find first static object / wall the bridge surface hits.
  (Development|PrintString (Utilities|String|ToString(Vector) _output_get))
  (bind (_outhit _returnvalue) (Collision|LineTraceForObjects (LocalVariables|GetStartLocationVar) (+ (LocalVariables|GetStartLocationVar) (* (LocalVariables|GetTraceDirectionVar) (LocalVariables|GetLineTraceLength))) (Utilities|Array|MakeArray "ObjectTypeQuery1" "ObjectTypeQuery8") false 0 "None"))
  (if _returnvalue
    ;[1 1 1] Line trace hit wall. Calculate bridge length and position.
    (LocalVariables|SetScalingFactorX (/ (.Distance (Collision|BreakHitResult _outhit)) (LocalVariables|GetDistanceToScaleConversionValue)))
    (LocalVariables|SetHalfwayVectorInWorldSpace (+ (LocalVariables|GetStartLocationVar) (/ (- (.Location (Collision|BreakHitResult _outhit)) (LocalVariables|GetStartLocationVar)) 2)))
    (else
      ;[1 1 1] Line trace didn't hit anything. Extend bridge to maximum length.
      (LocalVariables|SetScalingFactorX (/ (Variables|Default|GetMaxBridgeLength) (LocalVariables|GetDistanceToScaleConversionValue)))
      (LocalVariables|SetHalfwayVectorInWorldSpace (+ (LocalVariables|GetStartLocationVar) (* (LocalVariables|GetTraceDirectionVar) (/ (Variables|Default|GetMaxBridgeLength) 2.0))))))
  (Transformation|SetActorLocation (LocalVariables|GetSurfaveVar) (LocalVariables|GetHalfwayVectorInWorldSpace) false false)
  (Transformation|SetActorRelativeScale3D (LocalVariables|GetSurfaveVar) (Math|Vector|MakeVector (LocalVariables|GetScalingFactorX) (LocalVariables|GetScalingFactorY) 1.0)))