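; Reflective cube object for a Portal-style game, spawned by a cube dropper.
; When destroyed, it tells its parent dropper to drop a new cube if that dropper has auto-spawning enabled.
; BeginPlay shortens the tick interval, but Tick is empty.
; Logic to update the laser emitter when the cube moves is present but disconnected, so it never runs.
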(event EventBeginPlay
  (Actor|Tick|SetActorTickInterval 0.01))

(event Collision|EventActorBeginOverlap
  (params (OtherActor :type Actor%20Object%20Reference)))

(event EventTick
  (params (DeltaSeconds :type Float%20%28single-precision%29)))

(event EventDestroyed
  (bind _parentcubedropper (Variables|Default|GetParentCubeDropper))
  ;[1 1 1] Drop new cube, when being destroyed
  (Utilities|IsValid (Variables|Default|GetParentCubeDropper)
    (:Is%20Valid
      (if (Variables|/Game/Portals/Objects/CubeDropper_BP.CubeDropper_BP_C|GetAutoSpawnCubes _parentcubedropper)
        (Default|OnDropCubeEvent _parentcubedropper)))))

(fn ConstructionScript)