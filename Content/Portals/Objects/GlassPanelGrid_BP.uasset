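; GlassPanelGrid_BP is a construction-script actor that builds a grid of glass panels.
; Nested loops over the Z row count and Y column count place each panel by summing a per-row and per-column offset.
; Each panel is added as an unrotated, unit-scale instance on the GlassPanel instanced mesh component, and the event graph holds no active logic.
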(event EventBeginPlay)

(event Collision|EventActorBeginOverlap
  (params (OtherActor :type Actor%20Object%20Reference)))

(event EventTick
  (params (DeltaSeconds :type Float%20%28single-precision%29)))

(fn ConstructionScript
  ;[1 1 1] Height
  (for _index (range 0 (- (Variables|Default|GetNumAlongZ) 1))
    (LocalVariables|SetCurrentRow _index)
    (LocalVariables|SetCurrentRowOffset (* (Variables|Default|GetObjectOffsetZ) _index))
    ;[1 1 1] Width
    (for _index_2 (range 0 (- (Variables|Default|GetNumAlongY) 1))
      (LocalVariables|SetCurrentColumn _index_2)
      (LocalVariables|SetSpawnLocation (+ (* (Variables|Default|GetObjectOffsetY) (LocalVariables|GetCurrentColumn)) (LocalVariables|GetCurrentRowOffset)))
      (Components|InstancedStaticMesh|AddInstance (Variables|Default|GetGlassPanel) (Math|Transform|MakeTransform (LocalVariables|GetSpawnLocation) "0, 0, 0" "1,1,1")))))