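; Interactable pedestal button for the Portals game that signals listeners through an event dispatcher when used.
; Interact sets the activated light color, fires the dispatcher, then restores the deactivated color after ActivationDuration if that is above zero.
; Colors come from the MPC_Colors parameter collection, applied by SetLightColor through a new dynamic material instance on each call.
; The construction script starts the light deactivated, and CanBeInteractedWith returns the Enabled flag.
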(event EventBeginPlay)

(event Collision|EventActorBeginOverlap
  (params (OtherActor :type Actor%20Object%20Reference)))

(event EventTick
  (params (DeltaSeconds :type Float%20%28single-precision%29)))

(event EventInteract
  (bind _activationduration (Variables|Default|GetActivationDuration))
  (bind _returnvalue (Rendering|Material|GetVectorParameterValue "/Game/Portals/MPC_Colors.MPC_Colors" "PedestalButtonActivatedColor" :!class /Script/Engine.KismetMaterialLibrary))
  (CallFunction|SetLightColor _returnvalue)
  (Default|CallInteractEventDispatcher)
  (if (> _activationduration 0.0)
    (Utilities|FlowControl|Delay _activationduration)
    (bind _returnvalue_2 (Rendering|Material|GetVectorParameterValue "/Game/Portals/MPC_Colors.MPC_Colors" "PedestalButtonDeactivatedColor" :!class /Script/Engine.KismetMaterialLibrary))
    (CallFunction|SetLightColor _returnvalue_2)))

(fn ConstructionScript
  (bind _returnvalue (Rendering|Material|GetVectorParameterValue "/Game/Portals/MPC_Colors.MPC_Colors" "PedestalButtonDeactivatedColor" :!class /Script/Engine.KismetMaterialLibrary))
  (CallFunction|SetLightColor _returnvalue))

(fn SetLightColor
  (params (Color :type Linear%20Color%20Structure))
  (bind _returnvalue (Rendering|Material|CreateDynamicMaterialInstance (Variables|Default|GetPedestalButton) (Variables|Default|GetBlueLightMaterialIndex) "/Game/Portals/Models/PedestalButton/PedestalButton_BlueLight_mat.PedestalButton_BlueLight_mat" "None" :!class /Script/Engine.PrimitiveComponent))
  (Rendering|Material|SetVectorParameterValue _returnvalue "LightColor" Color :!class /Script/Engine.MaterialInstanceDynamic))

(fn CanbeInteractedwith
  (return (Variables|Default|GetEnabled)))