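; Weighted cube for the Portals game that the first-person character can pick up through its GrabberBP when Interact fires.
; On destruction it tells its parent cube dropper to drop a replacement if that dropper has AutoSpawnCubes enabled.
; SetCircleColor recolors the light circle through a dynamic material instance on the cube mesh.
; CanBeInteractedWith always returns false, even though Interact is implemented.
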(event Collision|EventActorBeginOverlap
  (params (OtherActor :type Actor%20Object%20Reference)))

(event EventTick
  (params (DeltaSeconds :type Float%20%28single-precision%29)))

(event EventInteract
  (bind _asfirst_person_character (Utilities|Casting|CastToFirstPersonCharacter (Game|GetPlayerCharacter 0)))
  (Default|Grab (Variables|/Game/FirstPersonCPP/Blueprints/FirstPersonCharacter.FirstPersonCharacter_C|GetGrabber_BP _asfirst_person_character) self))

(event EventDestroyed
  (bind _parentcubedropper (Variables|Default|GetParentCubeDropper))
  ;[1 1 1] Drop new cube, when being destroyed
  (Utilities|IsValid (Variables|Default|GetParentCubeDropper)
    (:Is%20Valid
      (if (Variables|/Game/Portals/Objects/CubeDropper_BP.CubeDropper_BP_C|GetAutoSpawnCubes _parentcubedropper)
        (Default|DropCubeEvent _parentcubedropper)))))

(fn ConstructionScript)

(fn SetCircleColor
  (params (Color :type Linear%20Color%20Structure))
  (bind _returnvalue (Rendering|Material|CreateDynamicMaterialInstance (Variables|Default|GetCube) (Variables|Default|GetLightCircleMaterialIndex) "/Game/Portals/Models/WeightedCube/WeightedCube_LightCircle_mat.WeightedCube_LightCircle_mat" "None" :!class /Script/Engine.PrimitiveComponent))
  (Rendering|Material|SetVectorParameterValue _returnvalue "CircleColor" Color :!class /Script/Engine.MaterialInstanceDynamic))

(fn CanbeInteractedwith
  (return false))